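; Base soldier enemy AI that turns to face the player and fires its child-actor gun on a repeating random delay.
; Tick drives the loop through latent Delays, pausing animation for a charge-up effect before each shot.
; Damage updates a 3D health bar; death notifies GameManager and EnemyManager, then explodes and destroys the actor.
; Shield defence, attack/defend decision logic and aim-tile spawning remain as disconnected or uncalled leftovers.
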(event Custom|Shoot
  ;[1 1 1] Shoot Me
  (if true
    _))

(event Custom|MeShoot
  ;[1 1 1] Shoot Me
  (Utilities|FlowControl|Sequence
    (:then_0
      (Variables|Default|SetIsShootingBP true)
      (bind _output_get (Variables|Default|SetLastCommand "NewEnumerator0"))
      (Utilities|Array|Add (Variables|Default|GetListOfCommands) _output_get))))

(event Custom|MeDefend
  ;[1 1 1] Shoot Me
)

(event Custom|TakeDamage
  (params (DamageToTake :type Integer))
  ;[1 1 1] Take Damage
  (bind _output_get (Variables|Default|SetHealth (- (Variables|Default|GetHealth) DamageToTake)))
  (bind _as3dhud (Utilities|Casting|CastTo3DHud (Variables|/Script/Engine.ChildActorComponent|GetChildActor (Variables|Default|Get3DHud))))
  (Default|TakeDamage _as3dhud DamageToTake))

(event Custom|MakeRandomDelay
  ;[1 1 1] Make Random Delay
  (Variables|Default|SetActionDelay (Math|Random|RandomFloatinRange 5.0 9.0)))

(event Custom|ChecksDeath
  ;[1 1 1] Checks Death
  (if (<= (Variables|Default|GetHealth) 0)
    (bind _outactors (Actor|GetAllActorsOfClass "/Game/BluePrints/Game_Necessary/GameManager.GameManager_C"))
    (Utilities|Array|RemoveItem (Variables|/Game/BluePrints/Game_Necessary/GameManager.GameManager_C|GetSpawnedEnemies (Utilities|Array|Get(acopy) _outactors)) self)
    (bind _outactors_2 (Actor|GetAllActorsOfClass "/Game/BluePrints/AI_Enemy_Stuff/EnemyManager.EnemyManager_C"))
    (Default|CheckNextRound (Utilities|Array|Get(acopy) _outactors_2))
    (Niagara|SpawnSystematLocation "/Game/Particles/EnemyDeathExplosion.EnemyDeathExplosion" (Transformation|GetWorldLocation (Variables|Debug|GetStaticMeshComponent)))
    (Actor|DestroyActor)))

(event EventTick
  (params (DeltaSeconds :type Float%20%28single-precision%29))
  (bind _skeletalmesh (Variables|Default|GetSkeletalMesh))
  ;[1 1 1] Logan Theatre Shooting
  (Utilities|FlowControl|Sequence
    (:then_0
      (CallFunction|ChecksDeath)
      (if true
        (CallFunction|MakeRandomDelay)
        (Default|ActivateMe (stale EventBeginPlay _asbase_gun))
        (Variables|Default|SetIsShootingBP true)
        (Utilities|FlowControl|Delay (Variables|Default|GetActionDelay))
        (Variables|/Script/Engine.SkeletalMeshComponent|SetbPauseAnims _skeletalmesh true)
        (bind _returnvalue (Audio|SpawnSoundAttached "/Game/Audio/Second_Semestar/SFX/EnemyChargeUp.EnemyChargeUp" (Variables|Default|GetGunPosition) "None" "0, 0, 0" "0, 0, 0" "KeepRelativeOffset" false 1.0 1.0 0.0 "/Game/BluePrints/AI_Enemy_Stuff/ChargeUp.ChargeUp" 0))
        (Audio|Components|Audio|Play _returnvalue 0.0)
        (bind _returnvalue_2 (Niagara|SpawnSystemAttached "/Game/Particles/EnemyChargeSystem.EnemyChargeSystem" (Variables|Default|GetGunPosition) "None" "0, 0, 0" "0, 0, 0" "KeepRelativeOffset" true))
        (Utilities|FlowControl|Delay 1.5)
        (Variables|/Script/Engine.SkeletalMeshComponent|SetbPauseAnims _skeletalmesh false)
        (bind _asbase_gun (Utilities|Casting|CastToBaseGun (Variables|/Script/Engine.ChildActorComponent|GetChildActor (Variables|Default|GetGunPosition))))
        (Default|ShootGun _asbase_gun)
        (Variables|Default|SetIsShootingBP false)
        (Utilities|FlowControl|Delay 0.6)))
    (:then_1
      (Transformation|SetActorRotation (Math|Conversions|RotationFromXVector (Math|Vector|RotateVector (Math|Vector|Normalize (* (- (Transformation|GetActorLocation (Game|Player|GetPlayerPawn 0)) (Transformation|GetActorLocation)) "1.000000,1.000000, 0")) "0, 0, 0"))))))

(event EventBeginPlay
  ;[1 1 1] Spawn Gun
  (Transformation|SetMobility "Movable")
  (bind _asbase_gun (Utilities|Casting|CastToBaseGun (Variables|/Script/Engine.ChildActorComponent|GetChildActor (Variables|Default|GetGunPosition))))
  (Default|ActivateMe _asbase_gun)
  (Variables|/Game/BluePrints/Guns/BaseGun.BaseGun_C|SetWhoOwnsMeGun _asbase_gun "NewEnumerator1")
  (bind _as3dhud (Utilities|Casting|CastTo3DHud (Variables|/Script/Engine.ChildActorComponent|GetChildActor (Variables|Default|Get3DHud))))
  (bind _output_get (Variables|/Game/BluePrints/UI_Stuff/3DHud.3DHud_C|SetMaxHealth _as3dhud (Variables|Default|GetMaxHealth)))
  (Variables|/Game/BluePrints/UI_Stuff/3DHud.3DHud_C|SetCurrentHealth _as3dhud _output_get)
  (Variables|/Game/BluePrints/UI_Stuff/3DHud.3DHud_C|SetHealthBarColor _as3dhud "(R=0.614583,G=0.006050,B=0.000000,A=1.000000)")
  (Default|SetHealthBarColor _as3dhud))

(event Input|KeyboardEvents|D
  (params (Key :type Key%20Structure))
  (:Pressed
    (CallFunction|MeDefend)))

(fn ConstructionScript)

(fn DetermineThreshold
  (bind _playercurrentlydefensive (Variables|Default|GetPlayerCurrentlyDefensive))
  (bind _shouldplaydefensive (Variables|Default|GetShouldPlayDefensive))
  (if (and _playercurrentlydefensive _shouldplaydefensive)
    (Variables|Default|SetThresholdFloat 5e+01) ; Player Is Defensive, AI should be Defensive
    (elif (and _playercurrentlydefensive (not _shouldplaydefensive))
      (Variables|Default|SetThresholdFloat 5e+01) ; Player is Defensive, AI should be Offensive
      (elif (and (not _playercurrentlydefensive) _shouldplaydefensive)
        (Variables|Default|SetThresholdFloat 5e+01) ; Player is Offensive, AI should be Defensive
        (elif (Math|Boolean|NANDBoolean _playercurrentlydefensive _shouldplaydefensive)
          (Variables|Default|SetThresholdFloat 5e+01) ; Player is Offensive, AI should be Offensive
        )))))

(fn DetermineState
  (if (< (Math|Random|RandomFloatinRange 0.0 99.0) (Variables|Default|GetThresholdFloat)) ; If the random number is above the threshold, the AI will play offensively. Otherwise it plays defensively.
    (Variables|Default|SetThisCurrentlyDefensive false)
    (else
      (Variables|Default|SetThisCurrentlyDefensive true))))

(fn SuggestState
  (bind _playerattackcount (Variables|Default|GetPlayerAttackCount))
  (bind _playerdefendcount (Variables|Default|GetPlayerDefendCount))
  (if (> _playerattackcount _playerdefendcount)
    (switch int _playerattackcount
      (:1
        (Variables|Default|SetShouldPlayDefensive true :!label _label))
      (:2
        (goto _label))
      (:5
        (Variables|Default|SetShouldPlayDefensive false :!label _label_2)))
    (else
      (switch int _playerdefendcount
        (:1
          (goto _label_2))
        (:2
          (goto _label))
        (:5
          (goto _label_2))))))

(fn MakeAimTiles
  (bind _aimdetectionspawn (Variables|Default|GetAimDetectionSpawn))
  (bind _numberforaimcube (Variables|Default|GetNumberForAimCube))
  (bind _relativelocation (Variables|/Script/Engine.SceneComponent|GetRelativeLocation _aimdetectionspawn))
  (for _index (range 0 (- (Variables|Default|GetAimGridRows) 1))
    (for _index_2 (range 0 (- (Variables|Default|GetAimGridColumns) 1))
      (Game|SpawnActorfromClass "/Game/BluePrints/AI_Enemy_Stuff/Aimdetection/AimDetectionCube_Blueprint.AimDetectionCube_Blueprint_C" (Math|Transform|MakeTransform (Math|Vector|MakeVector (+ (* _index _numberforaimcube) (- (.x _relativelocation) (/ (* (Variables|Default|GetAimGridRows) (Variables|Default|GetNumberForAimCube)) 2.0))) (.y _relativelocation) (+ (- (.z _relativelocation) (/ (* (Variables|Default|GetAimGridRows) (Variables|Default|GetNumberForAimCube)) 2.0)) (* _index_2 _numberforaimcube))) "0, 0, 0" "1,1,1") "AlwaysSpawn" 0 0))))