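; ActorAI is an enemy AI decision Blueprint that chooses between a defensive and non-defensive state by random roll.
; StartAI calls DetermineStateBool, which rolls against ThresholdFloat to set CurrentlyDefensive.
; SuggestAction sets ShouldAttackNotDefend from specific attack or defend counts, whichever is higher.
; DetermineThresholdFloat reads that flag and the opponent's stance, but every branch yields 50, and neither function is called here.
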(event EventBeginPlay)

(event Collision|EventActorBeginOverlap
  (params (OtherActor :type Actor%20Object%20Reference)))

(event EventTick
  (params (DeltaSeconds :type Float%20%28single-precision%29)))

(fn ConstructionScript)

(fn DetermineThresholdFloat
  (bind _opponentcurrentlydefensivebool (Variables|Default|GetOpponentCurrentlyDefensiveBool))
  (bind _shouldattacknotdefend (Variables|Default|GetShouldAttackNotDefend))
  (if (and _opponentcurrentlydefensivebool _shouldattacknotdefend)
    (Variables|Default|SetThresholdFloat 5e+01)
    (elif (and _opponentcurrentlydefensivebool (not _shouldattacknotdefend))
      (Variables|Default|SetThresholdFloat 5e+01)
      (elif (and (not _opponentcurrentlydefensivebool) _shouldattacknotdefend)
        (Variables|Default|SetThresholdFloat 5e+01)
        (elif (Math|Boolean|NANDBoolean _opponentcurrentlydefensivebool _shouldattacknotdefend)
          (Variables|Default|SetThresholdFloat 5e+01)))))
  (return))

(fn DetermineStateBool
  (if (< (Math|Random|RandomFloatinRange 0.0 99.0) (Variables|Default|GetThresholdFloat))
    (Variables|Default|SetCurrentlyDefensive false)
    (else
      (Variables|Default|SetCurrentlyDefensive true)))
  (return))

(fn SuggestAction
  (if (> (Variables|Default|GetEnemyAttackCount) (Variables|Default|GetEnemyDefendCount))
    (switch int (Variables|Default|GetEnemyAttackCount)
      (:1
        (Variables|Default|SetShouldAttackNotDefend false :!label _label))
      (:2
        (Variables|Default|SetShouldAttackNotDefend true :!label _label_2))
      (:5
        (goto _label)))
    (else
      (switch int (Variables|Default|GetEnemyDefendCount)
        (:1
          (goto _label))
        (:2
          (goto _label))
        (:5
          (goto _label_2))))))

(fn StartAI
  (CallFunction|DetermineStateBool))