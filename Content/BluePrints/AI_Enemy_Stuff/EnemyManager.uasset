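; Enemy wave manager that spawns each round's enemies evenly in a circle around the player and registers them with GameManager.
; WaveSpawner takes counts from AmountOfRounds, updates round text and music layers, and returns whether rounds are exhausted.
; SpawnWave plays round announcements, then MakeDelay leads into CircleSpawn, which mixes IsobotAI among soldiers in later rounds and spawns one medkit.
; Tick follows the player controller's location; R spawns soldiers at target points.
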(event Custom|MikeSpawner
  ;[1 1 1] MikeSpawn
)

(event Custom|CheckNextRound
  (if (>= 4 (Variables|Default|GetAmountSpawnedThisRound))
    (bind _outactors (Actor|GetAllActorsOfClass "/Game/BluePrints/Game_Necessary/GameManager.GameManager_C"))
    (Variables|/Game/BluePrints/Game_Necessary/GameManager.GameManager_C|SetcanSpawnNextRound (Utilities|Array|Get(acopy) _outactors) true)
    (else
      (Math|Integer|IncrementInt (Variables|Default|GetAmountSpawnedThisRound)))))

(event Custom|MakeDelay
  ;[1 1 1] Make Delay
  (switch int (Variables|Default|GetcurrentRound)
    (:Default
      (Utilities|FlowControl|Delay 4.0))
    (:0
      _)
    (:1
      _))
  (CallFunction|CircleSpawn))

(event Custom|SpawnHealthPack
  (if (not (Variables|Default|GethealthPackSpawned))
    (Variables|Default|SethealthPackSpawned true)
    (Game|SpawnActorfromClass "/Game/BluePrints/Medkit.Medkit_C" (Math|Transform|MakeTransform (Transformation|GetActorLocation (Variables|Default|GetHealthPackLocation)) "0,-180.000000, 0" "1,1,1") "Undefined" 0 0)))

(event EventBeginPlay)

(event Collision|EventActorBeginOverlap
  (params (OtherActor :type Actor%20Object%20Reference)))

(event EventTick
  (params (DeltaSeconds :type Float%20%28single-precision%29))
  (Transformation|SetActorLocation (Transformation|GetActorLocation (Game|GetPlayerController 0)) false false))

(event Input|KeyboardEvents|R
  (params (Key :type Key%20Structure))
  ;[1 1 1] MikeSpawn
  (:Pressed
    (for _array_element (Variables|Default|GetListOfEnemyTargetPoints)
      (bind _returnvalue (Game|SpawnActorfromClass "/Game/BluePrints/AI_Enemy_Stuff/BaseSoliderAI.BaseSoliderAI_C" (Transformation|GetActorTransform _array_element) "AlwaysSpawn" _array_element 0))
      (Utilities|Array|Add (Variables|Default|GetEnemyArray) _returnvalue))))

(fn ConstructionScript)

(fn CircleSpawn
  (bind _returnvalue (Game|Player|GetPlayerPawn 0))
  (bind _radiusfromcenter (Variables|Default|GetRadiusFromCenter))
  (bind _returnvalue_2 (Transformation|GetActorLocation _returnvalue))
  (CallFunction|SetAngle)
  (for _index (range 1 (Variables|Default|GetEnemyAmount))
    (CallFunction|SpawnHealthPack)
    (switch int (Variables|Default|GetcurrentRound)
      (:Default
        (switch int (Math|Random|RandomIntegerinRange 0 2)
          (:Default
            (bind _returnvalue_3 (Game|SpawnActorfromClass "/Game/BluePrints/AI_Enemy_Stuff/BaseSoliderAI.BaseSoliderAI_C" (Math|Transform|MakeTransform (Math|Vector|MakeVector (+ (.x _returnvalue_2) (* (Math|Trig|Sin(Radians) (* (Math|Conversions|ToFloat(Integer) _index) (Variables|Default|GetAngle))) _radiusfromcenter)) (+ (.y _returnvalue_2) (* _radiusfromcenter (Math|Trig|Cos(Radians) (* (Math|Conversions|ToFloat(Integer) _index) (Variables|Default|GetAngle))))) 325.0) (Math|Rotator|MakeRotator 0.0 0.0 (- (.yaw (Math|Rotator|FindLookatRotation (Math|Conversions|ToVector(Vector2D) (Math|Vector2D|MakeVector2D (+ (.x _returnvalue_2) (* (Math|Trig|Sin(Radians) (* (Math|Conversions|ToFloat(Integer) _index) (Variables|Default|GetAngle))) _radiusfromcenter)) (+ (.y _returnvalue_2) (* _radiusfromcenter (Math|Trig|Cos(Radians) (* (Math|Conversions|ToFloat(Integer) _index) (Variables|Default|GetAngle))))))) (Transformation|GetActorLocation self))) 9e+01)) "1,1,1") "Undefined" 0 0 :!label _label))
            (Niagara|SpawnSystemAttached "/Game/Particles/EnemySpawnSystem.EnemySpawnSystem" (Variables|/Game/BluePrints/AI_Enemy_Stuff/BaseSoliderAI.BaseSoliderAI_C|GetGunPosition _returnvalue_3) "None" "0, 0, 0" "0, 0, 0" "KeepRelativeOffset" false)
            (bind _outactors (Actor|GetAllActorsOfClass "/Game/BluePrints/Game_Necessary/GameManager.GameManager_C"))
            (Utilities|Array|Add (Variables|/Game/BluePrints/Game_Necessary/GameManager.GameManager_C|GetSpawnedEnemies (Utilities|Array|Get(acopy) _outactors)) _returnvalue_3))
          (:0
            (Game|SpawnActorfromClass "/Game/BluePrints/AI_Enemy_Stuff/IsobotAI.IsobotAI_C" (Math|Transform|MakeTransform (Math|Vector|MakeVector (+ (.x _returnvalue_2) (* (Math|Trig|Sin(Radians) (* (Math|Conversions|ToFloat(Integer) _index) (Variables|Default|GetAngle))) _radiusfromcenter)) (+ (.y _returnvalue_2) (* _radiusfromcenter (Math|Trig|Cos(Radians) (* (Math|Conversions|ToFloat(Integer) _index) (Variables|Default|GetAngle))))) 325.0) (Math|Rotator|MakeRotator 0.0 0.0 (- (.yaw (Math|Rotator|FindLookatRotation (Math|Conversions|ToVector(Vector2D) (Math|Vector2D|MakeVector2D (+ (.x _returnvalue_2) (* (Math|Trig|Sin(Radians) (* (Math|Conversions|ToFloat(Integer) _index) (Variables|Default|GetAngle))) _radiusfromcenter)) (+ (.y _returnvalue_2) (* _radiusfromcenter (Math|Trig|Cos(Radians) (* (Math|Conversions|ToFloat(Integer) _index) (Variables|Default|GetAngle))))))) (Transformation|GetActorLocation self))) 9e+01)) "1,1,1") "Undefined" 0 0)
            (bind _outactors_2 (Actor|GetAllActorsOfClass "/Game/BluePrints/Game_Necessary/GameManager.GameManager_C"))
            (Utilities|Array|Add (Variables|/Game/BluePrints/Game_Necessary/GameManager.GameManager_C|GetSpawnedEnemies (Utilities|Array|Get(acopy) _outactors_2)) 0))))
      (:0
        (goto _label))
      (:1
        (goto _label)))))

(fn SetAngle
  (Variables|Default|SetAngle (/ (* 2 (Math|Trig|GetPI)) (Math|Conversions|ToFloat(Integer) (Variables|Default|GetEnemyAmount)))))

(fn SpawnWave
  (params (AmountToSpawn :type Integer) (ForceAType :type Boolean) (ForcedEnemyTypes :type Array%20of%20Actor%20Object%20References))
  (switch int (Variables|Default|GetcurrentRound)
    (:Default
      _)
    (:0
      _)
    (:1
      (switch int (Math|Random|RandomIntegerinRange 0 1)
        (:0
          (Audio|PlaySound2D "/Game/Audio/VO_Audio/4_RoundTwo.4_RoundTwo" 1.0 1.0 0.0 0 0))
        (:1
          (Audio|PlaySound2D "/Game/Audio/VO_Audio/4_G_RoundTwo.4_G_RoundTwo" 1.0 1.0 0.0 0 0))))
    (:2
      (switch int (Math|Random|RandomIntegerinRange 0 1)
        (:0
          (Audio|PlaySound2D "/Game/Audio/VO_Audio/5_RoundThree.5_RoundThree" 1.0 1.0 0.0 0 0))
        (:1
          (Audio|PlaySound2D "/Game/Audio/VO_Audio/5_G_RoundThree.5_G_RoundThree" 1.0 1.0 0.0 0 0)))))
  (Variables|Default|SetEnemyAmount AmountToSpawn)
  (CallFunction|MakeDelay))

(fn WaveSpawner
  (bind _currentround (Variables|Default|GetcurrentRound))
  (if (>= (Utilities|Array|Length (Variables|Default|GetAmountOfRounds)) (Variables|Default|GetcurrentRound))
    (Utilities|FlowControl|Sequence
      (:then_0
        ;[1 1 1] Wave Spawner
        (CallFunction|SpawnWave (Utilities|Array|Get(acopy) (Variables|Default|GetAmountOfRounds) _currentround) false (Variables|Default|GetEnemyArray))
        (Math|Integer|IncrementInt _currentround
          (:%20%20
            (bind _outactors (Actor|GetAllActorsOfClass "/Game/BluePrints/UI_Stuff/ScreenText.ScreenText_C"))
            (for _array_element _outactors
              (bind _asscreen_text_ui (Utilities|Casting|CastToScreenTextUI (UserInterface|GetUserWidgetObject (Variables|/Game/BluePrints/UI_Stuff/ScreenText.ScreenText_C|GetWidget _array_element))))
              (Rendering|Components|TextRender|SetText (Variables|/Game/BluePrints/UI_Stuff/ScreenTextUI.ScreenTextUI_C|GetTextBlock_88 _asscreen_text_ui) (Utilities|Text|ToText(Integer) (Variables|Default|GetcurrentRound)))
              (if (== (Variables|Default|GetcurrentRound) 1)
                (bind _outactors_2 (Actor|GetAllActorsOfClass "/Game/BluePrints/Game_Necessary/AudioManager.AudioManager_C"))
                (Audio|Components|Audio|SetVolumeMultiplier (Variables|/Script/Engine.AmbientSound|GetAudioComponent (Variables|/Game/BluePrints/Game_Necessary/AudioManager.AudioManager_C|GetMusic2 (Utilities|Array|Get(acopy) _outactors_2))) 1.0 :!class /Script/Engine.AudioComponent)
                (elif (== (Variables|Default|GetcurrentRound) 2)
                  (bind _outactors_3 (Actor|GetAllActorsOfClass "/Game/BluePrints/Game_Necessary/AudioManager.AudioManager_C"))
                  (Audio|Components|Audio|SetVolumeMultiplier (Variables|/Script/Engine.AmbientSound|GetAudioComponent (Variables|/Game/BluePrints/Game_Necessary/AudioManager.AudioManager_C|GetMusic3 (Utilities|Array|Get(acopy) _outactors_3))) 1.0 :!class /Script/Engine.AudioComponent))))
            (return false))))
      (:then_1
        ;[1 1 1] Health Item Spawner
        (for _array_element_2 (Variables|Default|GetWavesThatHaveHealthItems)
          (if (== _array_element_2 (Variables|Default|GetcurrentRound))
            (Development|PrintString "Health Item Can Spawn")))))
    (else
      (return true))))