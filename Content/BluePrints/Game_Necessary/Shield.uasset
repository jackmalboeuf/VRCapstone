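; Shield actor that destroys soldier bullets on overlap or hit, with controller force feedback when player-owned.
; Activate/Deactivate toggle visibility and collision; Open/Close swap materials and play player-only animations.
; Once GameManager confirms pickup, opening starts timed active and cooldown phases, shown by timelines driving the CooldownCube's Height material parameter.
; In tutorial mode, player-owned hits count down TutorialHealth, then notify the tutorial TowerV3.
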(event Custom|DeactivateMe
  (bind _skeletalmesh (Variables|Default|GetSkeletalMesh))
  ;[1 1 1] Deactivate Me
  (Rendering|SetVisibility (Variables|Default|GetDefaultSceneRoot) false true)
  (Utilities|FlowControl|Delay 0.5)
  (Collision|SetCollisionEnabled _skeletalmesh "NoCollision")
  (Variables|/Script/Engine.PrimitiveComponent|SetbGenerateOverlapEvents _skeletalmesh false)
  (Collision|SetCollisionEnabled (Variables|Default|GetStaticMesh) "NoCollision"))

(event Custom|ActivateMe
  (bind _skeletalmesh (Variables|Default|GetSkeletalMesh))
  ;[1 1 1] Activate Me
  (bind _outactors (Actor|GetAllActorsOfClass "/Game/BluePrints/Game_Necessary/GameManager.GameManager_C"))
  (if (Variables|/Game/BluePrints/Game_Necessary/GameManager.GameManager_C|GetShieldHasBeenPickedUp (Utilities|Array|Get(acopy) _outactors))
    (if (Variables|Default|GethasSpawnedOnce)
      _
      (else
        (bind _outactors_2 (Actor|GetAllActorsOfClass "/Game/BluePrints/Game_Necessary/AudioManager.AudioManager_C"))
        (Default|VFXChanger (Utilities|Array|Get(acopy) _outactors_2) "Shield Activate")))
    (Variables|Default|SetHasStarted true)
    (Rendering|SetVisibility (Variables|Default|GetDefaultSceneRoot) true true)
    (Collision|SetCollisionEnabled _skeletalmesh "QueryAndPhysics")
    (Collision|SetCollisionEnabled (Variables|Default|GetStaticMesh) "QueryAndPhysics")
    (Variables|/Script/Engine.PrimitiveComponent|SetbGenerateOverlapEvents _skeletalmesh true)
    (Variables|Default|SethasSpawnedOnce true)))

(event Custom|Open%20Shield
  (bind _skeletalmesh (Variables|Default|GetSkeletalMesh))
  ;[1 1 1] Shield open and close
  (Rendering|Material|SetMaterial (Variables|Default|GetSkeletalMesh) 1 "/Game/Materials/ShieldClosedMat.ShieldClosedMat")
  (if (Utilities|Enum|Equal(Enum) (Variables|Default|GetWhoOwnsMe) "NewEnumerator0")
    (if (not (Variables|Default|GetIsCoolingDown))
      (Components|Animation|PlayAnimation _skeletalmesh "/Game/Models/Props/ShieldAnimations/SShield_Activation.SShield_Activation" false)
      (Collision|SetCollisionEnabled _skeletalmesh "QueryAndPhysics")
      (Variables|/Script/Engine.PrimitiveComponent|SetbGenerateOverlapEvents (Variables|Default|GetSkeletalMesh) true)
      (bind _outactors (Actor|GetAllActorsOfClass "/Game/BluePrints/Game_Necessary/GameManager.GameManager_C"))
      (if (Variables|/Game/BluePrints/Game_Necessary/GameManager.GameManager_C|GetShieldHasBeenPickedUp (Utilities|Array|Get(acopy) _outactors))
        (bind _outactors_2 (Actor|GetAllActorsOfClass "/Game/BluePrints/Game_Necessary/AudioManager.AudioManager_C"))
        (Default|VFXChanger (Utilities|Array|Get(acopy) _outactors_2) "ShieldOpen" (Transformation|GetWorldTransform (Variables|Default|GetStaticMesh)))
        (Variables|Default|SetIsCoolingDown true)
        (CallFunction|ShieldActiveDrain)
        (Utilities|FlowControl|Delay (Variables|Default|GetShieldActiveTime))
        (CallFunction|CloseShield)
        (CallFunction|ShieldCooldownRecharge)
        (Utilities|FlowControl|Delay (Variables|Default|GetShieldCooldown))
        (Variables|Default|SetIsCoolingDown false)))))

(event Custom|Close%20Shield
  (bind _skeletalmesh (Variables|Default|GetSkeletalMesh))
  ;[1 1 1] Shield open and close
  (Utilities|FlowControl|Delay 0.35)
  (Rendering|Material|SetMaterial (Variables|Default|GetSkeletalMesh) 0 "/Game/Materials/ShieldW_Transparencey.ShieldW_Transparencey")
  (if (Utilities|Enum|Equal(Enum) (Variables|Default|GetWhoOwnsMe) "NewEnumerator0")
    (Components|Animation|PlayAnimation _skeletalmesh "/Game/Models/Props/ShieldAnimations/SShield_Deactivation.SShield_Deactivation" false)
    (Collision|SetCollisionEnabled _skeletalmesh "NoCollision")
    (Variables|/Script/Engine.PrimitiveComponent|SetbGenerateOverlapEvents (Variables|Default|GetCooldownCube) false)))

(event Custom|ShieldCooldownRecharge
  ;[1 1 1] Shield Cooldown and Drain
  (bind _rechargevalue (Timeline|Recharge PlayFromStart)
    (:Update
      (Rendering|Material|SetScalarParameterValueonMaterials (Variables|Default|GetCooldownCube) "Height" (* _rechargevalue 9.0)))))

(event Custom|ShieldActiveDrain
  ;[1 1 1] Shield Cooldown and Drain
  (bind _drainvalue (Timeline|Drain PlayFromStart)
    (:Update
      (Rendering|Material|SetScalarParameterValueonMaterials (Variables|Default|GetCooldownCube) "Height" (* _drainvalue 9.0)))))

(event Custom|Tutorial%20Hit
  (bind _tutorialhealth (Variables|Default|GetTutorialHealth))
  ;[1 1 1] Tutorial Hit
  (Math|Integer|DecrementInt _tutorialhealth
    (:%20%20
      (if (<= _tutorialhealth 0)
        (Variables|Default|SetisTutorial false)
        (bind _outactors (Actor|GetAllActorsOfClass "/Game/BluePrints/Game_Necessary/TowerV3.TowerV3_C"))
        (for _array_element _outactors
          (if (Variables|/Game/BluePrints/Game_Necessary/TowerV3.TowerV3_C|GetIsTutorialTower _array_element)
            (Default|Tutorial:ShieldPartDone _array_element)))))))

(event Collision|EventHit
  (params (MyComp :type Primitive%20Component%20Object%20Reference) (Other :type Actor%20Object%20Reference) (OtherComp :type Primitive%20Component%20Object%20Reference) (bSelfMoved :type Boolean) (HitLocation :type Vector :default "0, 0, 0") (HitNormal :type Vector :default "0, 0, 0") (NormalImpulse :type Vector :default "0, 0, 0") (Hit :type Hit%20Result%20Structure%20%28by%20ref%29))
  ;[1 1 1] Begin Overlap: Bullet
  (bind _assoldier_bullet (Utilities|Casting|CastToSoldierBullet Other))
  (Actor|DestroyActor _assoldier_bullet)
  (switch Utilities|FlowControl|Switch|SwitchonOwner1 (Variables|Default|GetWhoOwnsMe)
    (:NewEnumerator0
      (Game|Feedback|ClientPlayForceFeedback (Game|GetPlayerController 0) "/Game/BluePrints/Game_Necessary/ShieldForceFeedback.ShieldForceFeedback" false false "None")
      (if (Variables|Default|GetisTutorial)
        (CallFunction|TutorialHit)))))

(event Collision|EventActorBeginOverlap
  (params (OtherActor :type Actor%20Object%20Reference))
  ;[1 1 1] Begin Overlap: Bullet
  (Utilities|Casting|CastToSoldierBullet OtherActor)
  (Math|Float|IncrementFloat (Variables|Default|GetCooldown)
    (:%20%20
      (Actor|DestroyActor OtherActor)
      (switch Utilities|FlowControl|Switch|SwitchonOwner1 (Variables|Default|GetWhoOwnsMe)
        (:NewEnumerator0
          (Game|Feedback|ClientPlayForceFeedback (Game|GetPlayerController 0) "/Game/BluePrints/Game_Necessary/ShieldForceFeedback.ShieldForceFeedback" false false "None")
          (if (Variables|Default|GetisTutorial)
            (CallFunction|TutorialHit)))))))

(event EventBeginPlay
  ;[1 1 1] Begin Play
  (CallFunction|CloseShield))

(fn ConstructionScript)