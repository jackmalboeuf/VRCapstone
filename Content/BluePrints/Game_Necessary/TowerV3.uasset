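; Damageable tower actor with an owner, doubling as a tutorial target that launches the battle.
; Hits from opposing BaseBullets lower Health, update the ball material's Height and screen health bars, play effects, and have GameManager check for a win.
; At zero health before the shield tutorial, a tutorial tower plays a level sequence, spawns the opponent prompt and starts enemy and battle through GameManager.
; A separate shield-done event spawns the destroy-tower win text.
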(event Custom|DeactivateMe
  ;[1 1 1] Activate/ Deactivate
  (Rendering|SetVisibility (Variables|Debug|GetStaticMeshComponent) false true))

(event Custom|ActivateMe
  ;[1 1 1] Activate/ Deactivate
  (Rendering|SetVisibility (Variables|Debug|GetStaticMeshComponent) true true))

(event Custom|TutorialTowerPartDone
  ;[1 1 1] Turorial Tower Part Done
  (if (Variables|Default|GetIsTutorialTower)
    (Development|SetHiddeninGame (Variables|Default|GetTextRender) true false)
    (Variables|Default|SetShieldTutorialHasStarted true)
    (bind _outactor (Sequencer|Player|CreateLevelSequencePlayer "/Game/OpeningLevel.OpeningLevel"))
    (Sequencer|Player|Play (Variables|/Script/LevelSequence.LevelSequenceActor|GetSequencePlayer _outactor) :!class /Script/MovieScene.MovieSceneSequencePlayer)
    (Game|SpawnActorfromClass "/Game/BluePrints/UI_Stuff/OpponentPrompt.OpponentPrompt_C" (Transformation|GetActorTransform (Variables|Default|GetOpponentPromptSpawn)) "Undefined" 0 0)
    (bind _outactors (Actor|GetAllActorsOfClass "/Game/BluePrints/Game_Necessary/GameManager.GameManager_C"))
    (Default|SpawnEnemy (Utilities|Array|Get(acopy) _outactors))
    (Default|StartBattle (Utilities|Array|Get(acopy) _outactors))))

(event Custom|MoveMe
  (bind _staticmeshcomponent (Variables|Debug|GetStaticMeshComponent))
  (bind _returnvalue (Transformation|GetWorldLocation _staticmeshcomponent))
  ;[1 1 1] MoveMe
  (Variables|Default|SetDefaultLocation (Math|Vector|MakeVector (.x _returnvalue) (.y _returnvalue) (.z _returnvalue)))
  (Transformation|SetWorldLocation _staticmeshcomponent (Math|Vector|MakeVector (+ (.x _returnvalue) 1e+02) 0.0 0.0) false false)
  (Utilities|FlowControl|Delay 0.1)
  (Transformation|SetWorldLocation _staticmeshcomponent (Math|Vector|MakeVector (- (.x (Variables|Default|GetDefaultLocation)) 1e+02) 0.0 0.0) false false))

(event Custom|Tutorial:%20Shield%20Part%20Done
  ;[1 1 1] Tutorial Shield Part Done
  (Variables|Default|SetTutorialHasEnded true)
  (Game|SpawnActorfromClass "/Game/BluePrints/UI_Stuff/DestroyTowerWinText.DestroyTowerWinText_C" (Transformation|GetActorTransform (Variables|Default|GetWinTutorialSpawn)) "Undefined" 0 0))

(event Collision|EventHit
  (params (MyComp :type Primitive%20Component%20Object%20Reference) (Other :type Actor%20Object%20Reference) (OtherComp :type Primitive%20Component%20Object%20Reference) (bSelfMoved :type Boolean) (HitLocation :type Vector :default "0, 0, 0") (HitNormal :type Vector :default "0, 0, 0") (NormalImpulse :type Vector :default "0, 0, 0") (Hit :type Hit%20Result%20Structure%20%28by%20ref%29))
  ;[1 1 1] Bullet Hit
  (if (Variables|Default|GetCanTakeDamage)
    (bind _asbase_bullet (Utilities|Casting|CastToBaseBullet (stale Collision|EventActorBeginOverlap OtherActor)))
    (if (not (Utilities|Enum|Equal(Enum) (Variables|Default|GetWhoOwnsMe) (Variables|/Game/BluePrints/Guns/BaseBullet.BaseBullet_C|GetWhoOwnsMeBullet _asbase_bullet)))
      (Development|PrintString "Tower Was Hit")
      (bind _output_get (Variables|Default|SetHealth (- (Variables|Default|GetHealth) 1.0)))
      (Rendering|Material|SetScalarParameterValueonMaterials (Variables|Default|GetTowerBall) "Height" (* (Math|Float|NormalizetoRange _output_get 0.0 (Variables|Default|GetMaxHealth)) 7.5e+02))
      (for _array_element (Variables|Default|GetScreenHealthBars)
        (Default|UpdateHealth _array_element (Math|Float|NormalizetoRange (Variables|Default|GetHealth) 0.0 (Variables|Default|GetMaxHealth))))
      (Utilities|FlowControl|Sequence
        (:then_0
          (bind _outactors (Actor|GetAllActorsOfClass "/Game/BluePrints/Game_Necessary/GameManager.GameManager_C"))
          (Default|CheckWin (Utilities|Array|Get(acopy) _outactors))
          (if (<= (Variables|Default|GetHealth) 0.0)
            (if (not (Variables|Default|GetShieldTutorialHasStarted))
              (CallFunction|TutorialTowerPartDone))))
        (:then_1
          (switch Utilities|FlowControl|Switch|SwitchonOwner (Variables|Default|GetWhoOwnsMe)
            (:NewEnumerator0
              (Game|Feedback|ClientPlayForceFeedback (Game|GetPlayerController 0) "/Game/ControllerFailedShot.ControllerFailedShot" false false "None"))))
        (:then_2
          (Effects|SpawnEmitterAttached "/Game/StarterContent/Particles/P_Explosion.P_Explosion" 0 "None"))
        (:then_3
          (Audio|PlaySoundatLocation "/Game/Audio/10_26/VR_Tower_Hit_Successful.VR_Tower_Hit_Successful" (Transformation|GetWorldLocation (Variables|Debug|GetStaticMeshComponent)) "0, 0, 0" 1.0 1.0 0.0 0 0 0))))))

(event EventBeginPlay
  ;[1 1 1] Begin Play
  (Rendering|Material|SetScalarParameterValueonMaterials (Variables|Default|GetTowerBall) "Height" (* (Math|Float|NormalizetoRange (Variables|Default|GetHealth) 0.0 (Variables|Default|GetMaxHealth)) 1.25e+03))
  (if (Variables|Default|GetIsTutorialTower)
    (Development|SetHiddeninGame (Variables|Default|GetTextRender) false false)))

(event EventTick
  (params (DeltaSeconds :type Float%20%28single-precision%29))
  ;[1 1 1] TICK: Removes Text from Player "Tower"
  (Utilities|FlowControl|Sequence
    (:then_0
      (if (not (Variables|Default|GetIsTutorialTower))
        (if (Utilities|Enum|Equal(Enum) (Variables|Default|GetWhoOwnsMe) "NewEnumerator0")
          (Rendering|SetVisibility (Variables|Default|GetTextRender) false false))))
    (:then_1
      (if (Variables|Default|GetTutorialHasEnded)
        (if (<= (Variables|Default|GetHealth) 0.0)
          (Variables|Default|SetHealth 0.0))))))

(event Collision|EventActorBeginOverlap
  (params (OtherActor :type Actor%20Object%20Reference))
  ;[1 1 1] Bullet Hit
  (if (Variables|Default|GetCanTakeDamage)
    (bind _asbase_bullet (Utilities|Casting|CastToBaseBullet OtherActor))
    (if (not (Utilities|Enum|Equal(Enum) (Variables|Default|GetWhoOwnsMe) (Variables|/Game/BluePrints/Guns/BaseBullet.BaseBullet_C|GetWhoOwnsMeBullet _asbase_bullet)))
      (Development|PrintString "Tower Was Hit")
      (bind _output_get (Variables|Default|SetHealth (- (Variables|Default|GetHealth) 1.0)))
      (Rendering|Material|SetScalarParameterValueonMaterials (Variables|Default|GetTowerBall) "Height" (* (Math|Float|NormalizetoRange _output_get 0.0 (Variables|Default|GetMaxHealth)) 7.5e+02))
      (for _array_element (Variables|Default|GetScreenHealthBars)
        (Default|UpdateHealth _array_element (Math|Float|NormalizetoRange (Variables|Default|GetHealth) 0.0 (Variables|Default|GetMaxHealth))))
      (Utilities|FlowControl|Sequence
        (:then_0
          (bind _outactors (Actor|GetAllActorsOfClass "/Game/BluePrints/Game_Necessary/GameManager.GameManager_C"))
          (Default|CheckWin (Utilities|Array|Get(acopy) _outactors))
          (if (<= (Variables|Default|GetHealth) 0.0)
            (if (not (Variables|Default|GetShieldTutorialHasStarted))
              (CallFunction|TutorialTowerPartDone))))
        (:then_1
          (switch Utilities|FlowControl|Switch|SwitchonOwner (Variables|Default|GetWhoOwnsMe)
            (:NewEnumerator0
              (Game|Feedback|ClientPlayForceFeedback (Game|GetPlayerController 0) "/Game/ControllerFailedShot.ControllerFailedShot" false false "None"))))
        (:then_2
          (Effects|SpawnEmitterAttached "/Game/StarterContent/Particles/P_Explosion.P_Explosion" 0 "None"))
        (:then_3
          (Audio|PlaySoundatLocation "/Game/Audio/10_26/VR_Tower_Hit_Successful.VR_Tower_Hit_Successful" (Transformation|GetWorldLocation (Variables|Debug|GetStaticMeshComponent)) "0, 0, 0" 1.0 1.0 0.0 0 0 0))))))

(event Input|KeyboardEvents|8
  (params (Key :type Key%20Structure))
  ;[1 1 1] Bullet Hit
  (:Pressed
    (if (Variables|Default|GetCanTakeDamage)
      (bind _asbase_bullet (Utilities|Casting|CastToBaseBullet (stale Collision|EventActorBeginOverlap OtherActor)))
      (if (not (Utilities|Enum|Equal(Enum) (Variables|Default|GetWhoOwnsMe) (Variables|/Game/BluePrints/Guns/BaseBullet.BaseBullet_C|GetWhoOwnsMeBullet _asbase_bullet)))
        (Development|PrintString "Tower Was Hit")
        (bind _output_get (Variables|Default|SetHealth (- (Variables|Default|GetHealth) 1.0)))
        (Rendering|Material|SetScalarParameterValueonMaterials (Variables|Default|GetTowerBall) "Height" (* (Math|Float|NormalizetoRange _output_get 0.0 (Variables|Default|GetMaxHealth)) 7.5e+02))
        (for _array_element (Variables|Default|GetScreenHealthBars)
          (Default|UpdateHealth _array_element (Math|Float|NormalizetoRange (Variables|Default|GetHealth) 0.0 (Variables|Default|GetMaxHealth))))
        (Utilities|FlowControl|Sequence
          (:then_0
            (bind _outactors (Actor|GetAllActorsOfClass "/Game/BluePrints/Game_Necessary/GameManager.GameManager_C"))
            (Default|CheckWin (Utilities|Array|Get(acopy) _outactors))
            (if (<= (Variables|Default|GetHealth) 0.0)
              (if (not (Variables|Default|GetShieldTutorialHasStarted))
                (CallFunction|TutorialTowerPartDone))))
          (:then_1
            (switch Utilities|FlowControl|Switch|SwitchonOwner (Variables|Default|GetWhoOwnsMe)
              (:NewEnumerator0
                (Game|Feedback|ClientPlayForceFeedback (Game|GetPlayerController 0) "/Game/ControllerFailedShot.ControllerFailedShot" false false "None"))))
          (:then_2
            (Effects|SpawnEmitterAttached "/Game/StarterContent/Particles/P_Explosion.P_Explosion" 0 "None"))
          (:then_3
            (Audio|PlaySoundatLocation "/Game/Audio/10_26/VR_Tower_Hit_Successful.VR_Tower_Hit_Successful" (Transformation|GetWorldLocation (Variables|Debug|GetStaticMeshComponent)) "0, 0, 0" 1.0 1.0 0.0 0 0 0)))))))

(fn ConstructionScript)