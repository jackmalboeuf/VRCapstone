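; Audio manager that plays battle music and gun, shield, elevator and impact sound effects by type.
; VFXChanger moves one shared VFXGenerator to the given transform to play a sound, some shield sounds randomised, and drops requests while the Tick-polled flag reads playing.
; MusicChanger puts intro or base, round and spice loops on three separate players for layering, while win or lose stops all three before playing its track.
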(event Custom|MusicChanger
  (params (TypeOfMusic :type String))
  (bind _music2 (Variables|Default|GetMusic2))
  (bind _music (Variables|Default|GetMusic))
  (bind _music3 (Variables|Default|GetMusic3))
  (bind _music_2 (Variables|Default|GetMusic))
  (bind _audiocomponent (Variables|/Script/Engine.AmbientSound|GetAudioComponent _music))
  (bind _audiocomponent_2 (Variables|/Script/Engine.AmbientSound|GetAudioComponent _music2))
  (bind _audiocomponent_3 (Variables|/Script/Engine.AmbientSound|GetAudioComponent _music3))
  (bind _audiocomponent_4 (Variables|/Script/Engine.AmbientSound|GetAudioComponent _music_2))
  (Development|PrintString "Music Called")
  (switch string TypeOfMusic
    (:PlayerLoose
      (Audio|Components|Audio|Stop _audiocomponent)
      (Audio|Components|Audio|SetSound (Variables|/Script/Engine.AmbientSound|GetAudioComponent (Variables|Default|GetMusic)) "/Game/Audio/Second_Semestar/Music/Loss/lose__02_08_2019_.lose__02_08_2019_")
      (Audio|Components|Audio|Play _audiocomponent 0.0))
    (:PlayerWin
      (Audio|Components|Audio|Stop _audiocomponent)
      (Audio|Components|Audio|SetSound (Variables|/Script/Engine.AmbientSound|GetAudioComponent (Variables|Default|GetMusic)) "/Game/Audio/Second_Semestar/Music/Win/victory_grunge__02_08_2019_.victory_grunge__02_08_2019_")
      (Audio|Components|Audio|Play _audiocomponent 0.0))
    (:Base
      (Audio|Components|Audio|SetSound (Variables|/Script/Engine.AmbientSound|GetAudioComponent (Variables|Default|GetMusic)) "/Game/Audio/Second_Semestar/Music/General/layers_cut/battleMusic_BaseLoop_01__02_08_19_.battleMusic_BaseLoop_01__02_08_19_")
      (Audio|Components|Audio|Play _audiocomponent 0.0))
    (:Round1
      (Audio|Components|Audio|SetSound _audiocomponent_2 "/Game/Audio/Second_Semestar/Music/General/layers_cut/battleMusic_RoundLoop_01__02_08_2019_.battleMusic_RoundLoop_01__02_08_2019_")
      (Audio|Components|Audio|Play _audiocomponent_2 0.0))
    (:Spice
      (Audio|Components|Audio|SetSound _audiocomponent_3 "/Game/Audio/Second_Semestar/Music/General/layers_cut/battleMusic_SpiceLoop_01__02_08_2019_.battleMusic_SpiceLoop_01__02_08_2019_")
      (Audio|Components|Audio|Play _audiocomponent_3 0.0))
    (:IntroStart
      (Audio|Components|Audio|SetSound _audiocomponent_4 "/Game/Audio/Second_Semestar/Music/General/layers_cut/battleMusic_BaseIntro_01__02_08_19_.battleMusic_BaseIntro_01__02_08_19_")
      (Audio|Components|Audio|Play _audiocomponent_4 0.0))))

(event Custom|VFX%20Changer
  (params (Type%20of%20Sound :type String) (Location :type Transform))
  (bind _vfxgenerator (Variables|Default|GetVFXGenerator))
  (bind _vfxgenerator_2 (Variables|Default|GetVFXGenerator))
  (bind _vfxgenerator_3 (Variables|Default|GetVFXGenerator))
  (bind _vfxgenerator_4 (Variables|Default|GetVFXGenerator))
  (bind _vfxgenerator_5 (Variables|Default|GetVFXGenerator))
  (bind _vfxgenerator_6 (Variables|Default|GetVFXGenerator))
  (bind _vfxgenerator_7 (Variables|Default|GetVFXGenerator))
  (bind _vfxgenerator_8 (Variables|Default|GetVFXGenerator))
  (bind _vfxgenerator_9 (Variables|Default|GetVFXGenerator))
  (bind _vfxgenerator_10 (Variables|Default|GetVFXGenerator))
  (bind _vfxgenerator_11 (Variables|Default|GetVFXGenerator))
  (bind _vfxgenerator_12 (Variables|Default|GetVFXGenerator))
  (bind _vfxgenerator_13 (Variables|Default|GetVFXGenerator))
  (bind _audiocomponent (Variables|/Script/Engine.AmbientSound|GetAudioComponent _vfxgenerator_3))
  (bind _audiocomponent_2 (Variables|/Script/Engine.AmbientSound|GetAudioComponent _vfxgenerator_9))
  (bind _audiocomponent_3 (Variables|/Script/Engine.AmbientSound|GetAudioComponent _vfxgenerator_10))
  (bind _audiocomponent_4 (Variables|/Script/Engine.AmbientSound|GetAudioComponent _vfxgenerator_2))
  (bind _audiocomponent_5 (Variables|/Script/Engine.AmbientSound|GetAudioComponent _vfxgenerator_12))
  (bind _audiocomponent_6 (Variables|/Script/Engine.AmbientSound|GetAudioComponent _vfxgenerator_13))
  (Development|PrintString "VFX Changer")
  (if (not (Variables|Default|GetisVFXPlaying))
    (switch string Type%20of%20Sound
      (:GunInvalid
        (Transformation|SetActorTransform _vfxgenerator_6 Location)
        (Audio|Components|Audio|SetSound (Variables|/Script/Engine.AmbientSound|GetAudioComponent _vfxgenerator_6) "/Game/Audio/Second_Semestar/SFX/VR_Player_Gun/Gun_Invalid.Gun_Invalid")
        (Audio|Components|Audio|Play _audiocomponent_4 0.0))
      (:Shield%20Activate
        (switch int (Math|Random|RandomIntegerinRange 0 2)
          (:0
            (Transformation|SetActorTransform _vfxgenerator_4 Location)
            (Audio|Components|Audio|SetSound (Variables|/Script/Engine.AmbientSound|GetAudioComponent _vfxgenerator_4) "/Game/Audio/Second_Semestar/SFX/VR_Player_Shield/ShieldActivate.ShieldActivate")
            (Audio|Components|Audio|Play _audiocomponent_4 0.0))
          (:1
            (Transformation|SetActorTransform _vfxgenerator_5 Location)
            (Audio|Components|Audio|SetSound (Variables|/Script/Engine.AmbientSound|GetAudioComponent _vfxgenerator_5) "/Game/Audio/Second_Semestar/SFX/VR_Player_Shield/ShieldActivate_2.ShieldActivate_2")
            (Audio|Components|Audio|Play _audiocomponent_4 0.0))
          (:2
            (Transformation|SetActorTransform _vfxgenerator Location)
            (Audio|Components|Audio|SetSound (Variables|/Script/Engine.AmbientSound|GetAudioComponent _vfxgenerator) "/Game/Audio/Second_Semestar/SFX/VR_Player_Shield/ShieldActivate_3.ShieldActivate_3")
            (Audio|Components|Audio|Play _audiocomponent_4 0.0))))
      (:Gun%20Charge%20Reverse
        (Transformation|SetActorTransform _vfxgenerator_7 Location)
        (Audio|Components|Audio|SetSound (Variables|/Script/Engine.AmbientSound|GetAudioComponent _vfxgenerator_7) "/Game/Audio/Second_Semestar/SFX/VR_Player_Gun/Gun_ChargeUpReverse.Gun_ChargeUpReverse")
        (Audio|Components|Audio|Play _audiocomponent_4 0.0))
      (:ElevatorUpDoorClose
        (Transformation|SetActorTransform _vfxgenerator_8 Location)
        (Audio|Components|Audio|SetSound (Variables|/Script/Engine.AmbientSound|GetAudioComponent _vfxgenerator_8) "/Game/Audio/Second_Semestar/SFX/Elevator_MatchedToMovie/VR_ElevatorUp_DoorClose.VR_ElevatorUp_DoorClose")
        (Audio|Components|Audio|Play _audiocomponent_4 0.0))
      (:ShieldPopUp
        (switch int (Math|Random|RandomIntegerinRange 0 1)
          (:0
            (Transformation|SetActorTransform _vfxgenerator_9 Location)
            (Audio|Components|Audio|SetSound _audiocomponent_2 "/Game/Audio/Second_Semestar/SFX/VR_Player_Shield/ShieldPop.ShieldPop")
            (Audio|Components|Audio|Play _audiocomponent_2 0.0))
          (:1
            (Transformation|SetActorTransform _vfxgenerator_10 Location)
            (Audio|Components|Audio|SetSound _audiocomponent_3 "/Game/Audio/Second_Semestar/SFX/VR_Player_Shield/ShieldPop_1.ShieldPop_1")
            (Audio|Components|Audio|Play _audiocomponent_3 0.0))))
      (:GunChargeUp
        (Transformation|SetActorTransform _vfxgenerator_11 Location)
        (Audio|Components|Audio|SetSound (Variables|/Script/Engine.AmbientSound|GetAudioComponent _vfxgenerator_11) "/Game/Audio/First_Semestar/10_26/VR_Unit_Gun_Shot.VR_Unit_Gun_Shot")
        (Audio|Components|Audio|Play _audiocomponent_4 0.0))
      (:GunFizzle
        (Transformation|SetActorTransform _vfxgenerator_12 Location)
        (Audio|Components|Audio|SetSound _audiocomponent_5 "/Game/Audio/Second_Semestar/SFX/VR_Player_Gun/Gun_Fizzle.Gun_Fizzle")
        (Audio|Components|Audio|Play _audiocomponent_5 0.0))
      (:BulletHit
        (Transformation|SetActorTransform _vfxgenerator_3 Location)
        (Audio|Components|Audio|SetSound _audiocomponent "/Game/Audio/First_Semestar/Pre_10_26/VR_LazerGunImpact.VR_LazerGunImpact")
        (Audio|Components|Audio|Play _audiocomponent 0.0))
      (:ShieldOpen
        (Transformation|SetActorTransform _vfxgenerator_13 Location)
        (Audio|Components|Audio|SetSound _audiocomponent_6 "/Game/Audio/Second_Semestar/SFX/VR_Player_Shield/ShieldActivate.ShieldActivate")
        (Audio|Components|Audio|Play _audiocomponent_6 0.0)))))

(event EventTick
  (params (DeltaSeconds :type Float%20%28single-precision%29))
  (Variables|Default|SetisMusicPlaying (Audio|Components|Audio|IsPlaying (Variables|/Script/Engine.AmbientSound|GetAudioComponent (Variables|Default|GetMusic))))
  (Variables|Default|SetisVFXPlaying (Audio|Components|Audio|IsPlaying (Variables|/Script/Engine.AmbientSound|GetAudioComponent (Variables|Default|GetVFXGenerator)))))

(fn ConstructionScript)