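; Board tile actor for a grid board that tracks its row, column and owning player, and whether a character can be placed on it.
; A BaseGun overlap on an unoccupied tile swaps the mesh to a highlight material and enables placement; ending overlap reverts both.
; Setter events assign one of four rows, three columns or two owners through enums.
; Tick refreshes a debug text showing owner, row and column.
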(event Custom|Set%20Player%201%20as%20Owner
  ;[1 1 1] Set Player 1 as Owner
  (Variables|Default|SetHasOwner "NewEnumerator0"))

(event Custom|Set%20Player%202%20as%20Owner
  ;[1 1 1] Set Player 2 as Owner
  (Variables|Default|SetHasOwner "NewEnumerator1"))

(event Custom|DebugTextForTiles
  ;[1 1 1] Debug Text for Tiles
  (Rendering|Components|TextRender|SetText (Variables|Default|GetNumber) (Utilities|Text|ToText(String) (Utilities|String|Append (Utilities|String|EnumtoString (Variables|Default|GetHasOwner)) "<br>" (Utilities|String|EnumtoString (Variables|Default|GetTile%20Number)) "<br>" (Utilities|String|EnumtoString (Variables|Default|GetTile%20Column%20Number))))))

(event Custom|SetLocationAsRow1
  ;[1 1 1] Set Location as Row 1
  (Variables|Default|SetTile%20Number "NewEnumerator0"))

(event Custom|SetLocationAsRow2
  ;[1 1 1] Set Location as Row 2
  (Variables|Default|SetTile%20Number "NewEnumerator1"))

(event Custom|SetLocationAsRow3
  ;[1 1 1] Set Location as Row 3
  (Variables|Default|SetTile%20Number "NewEnumerator2"))

(event Custom|SetLocationAsColumn1
  ;[1 1 1] Set Location as Column 1
  (Variables|Default|SetTile%20Column%20Number "NewEnumerator0"))

(event Custom|SetLocationAsColumn2
  ;[1 1 1] Set Location as Column 2
  (Variables|Default|SetTile%20Column%20Number "NewEnumerator1"))

(event Custom|SetLocationAsColumn3
  ;[1 1 1] Set Location as Column 3
  (Variables|Default|SetTile%20Column%20Number "NewEnumerator2"))

(event Custom|SetLocationAsRow4
  ;[1 1 1] Set Location as Row 4
  (Variables|Default|SetTile%20Number "NewEnumerator3"))

(event EventTick
  (params (DeltaSeconds :type Float%20%28single-precision%29))
  (CallFunction|DebugTextforTiles))

(event Collision|EventActorBeginOverlap
  (params (OtherActor :type Actor%20Object%20Reference))
  (Utilities|Casting|CastToBaseGun OtherActor)
  (if (not (Variables|Default|GetCharacterOnMe))
    (Rendering|Material|SetMaterial (Variables|Debug|GetStaticMeshComponent) 0 "/Game/Materials/DarkBlueMetallic.DarkBlueMetallic")
    (Variables|Default|SetCanPlaceCharacter true)))

(event Collision|EventActorEndOverlap
  (params (OtherActor :type Actor%20Object%20Reference))
  (Utilities|Casting|CastToBaseGun OtherActor)
  (Rendering|Material|SetMaterial (Variables|Debug|GetStaticMeshComponent) 0 "/Game/Materials/BlackBox.BlackBox")
  (Variables|Default|SetCanPlaceCharacter false))

(fn ConstructionScript)