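; Shield actor that can be switched on and off and absorbs bullet hits.
; ActivateMe and DeactivateMe toggle the root's visibility, propagated to children, along with the shield mesh's collision.
; On overlap with an actor whose class is exactly BaseBullet, it subtracts the bullet's Damage from Health and destroys the bullet.
; Health depletion is not handled in this graph.
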(event Custom|DeactivateMe
  (Rendering|SetVisibility (Variables|Default|GetDefaultSceneRoot) false true)
  (Collision|SetCollisionEnabled (Variables|Default|GetShieldMesh) "NoCollision"))

(event Custom|ActivateMe
  (Rendering|SetVisibility (Variables|Default|GetDefaultSceneRoot) true true)
  (Collision|SetCollisionEnabled (Variables|Default|GetShieldMesh) "QueryAndPhysics"))

(event EventBeginPlay)

(event Collision|EventActorBeginOverlap
  (params (OtherActor :type Actor%20Object%20Reference))
  (if (== (Utilities|GetClass OtherActor) "/Game/BluePrints/Guns/BaseBullet.BaseBullet_C")
    (bind _asbase_bullet (Utilities|Casting|CastToBaseBullet OtherActor))
    (Variables|Default|SetHealth (- (Variables|Default|GetHealth) (Math|Conversions|ToFloat(Integer) (Variables|/Game/BluePrints/Guns/BaseBullet.BaseBullet_C|GetDamage _asbase_bullet))))
    (Actor|DestroyActor OtherActor)))

(event EventTick
  (params (DeltaSeconds :type Float%20%28single-precision%29)))

(fn ConstructionScript)