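; Base soldier AI Blueprint that spawns a gun and shield as child actors and either shoots or defends.
; Once started, Tick repeatedly fires the gun through an action delay.
; A separate Shoot event randomly picks shooting or defending, partly based on the last command.
; Each action is logged to a command list and printed, with defending briefly activating the shield.
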(event Custom|Shoot
  ;[1 1 1] Shoot Me
  (if (< (Math|Random|RandomInteger 100) 6)
    (CallFunction|MeShoot)
    (elif (> (Math|Random|RandomInteger 5) 3)
      (if (Utilities|Enum|Equal(Enum) (Variables|Default|GetLastCommand) "NewEnumerator1")
        (CallFunction|MeDefend)
        (else
          (CallFunction|MeDefend)))
      (elif (Utilities|Enum|Equal(Enum) (Variables|Default|GetLastCommand) "NewEnumerator0")
        (CallFunction|MeDefend)
        (else
          (CallFunction|MeShoot))))))

(event Custom|MeShoot
  (Utilities|FlowControl|Sequence
    (:then_0
      (bind _output_get (Variables|Default|SetLastCommand "NewEnumerator0"))
      (Utilities|Array|Add (Variables|Default|GetListOfCommands) _output_get))
    (:then_1
      (Development|PrintString "Solider is Shooting")
      (bind _asbase_gun (Utilities|Casting|CastToBaseGun (Variables|/Script/Engine.ChildActorComponent|GetChildActor (Variables|Default|GetGunPosition))))
      (Default|ShootGun _asbase_gun))))

(event Custom|MeDefend
  (Utilities|FlowControl|Sequence
    (:then_0
      (bind _output_get (Variables|Default|SetLastCommand "NewEnumerator1"))
      (Utilities|Array|Add (Variables|Default|GetListOfCommands) _output_get))
    (:then_1
      (Development|PrintString "Solider is Defending")
      (bind _asshield (Utilities|Casting|CastToShield (Variables|/Script/Engine.ChildActorComponent|GetChildActor (Variables|Default|GetShieldPosition))))
      (Default|ActivateMe _asshield)
      (Utilities|FlowControl|Delay 0.2)
      (Default|DeactivateMe _asshield))))

(event EventTick
  (params (DeltaSeconds :type Float%20%28single-precision%29))
  (if (Variables|Default|GetHasStarted)
    (Utilities|FlowControl|Delay (Variables|Default|GetActionDelay))
    (CallFunction|MeShoot)))

(event EventBeginPlay
  ;[1 1 1] Spawn Gun
  (ChildActorComponent|SetChildActorClass (Variables|Default|GetGunPosition) (Variables|Default|GetCurrentGun))
  (bind _asshield (Utilities|Casting|CastToShield (Variables|/Script/Engine.ChildActorComponent|GetChildActor (Variables|Default|GetShieldPosition))))
  (Default|DeactivateMe _asshield))

(fn ConstructionScript)