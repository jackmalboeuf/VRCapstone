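; Base gun projectile for a VR game that damages soldier AI or the player and expires after a countdown.
; Hit and overlap share one cast chain that ignores motion controllers and guns, using an owner enum to gate soldier damage.
; Impacts spawn sound, explosion and decal, but only player hits destroy the bullet immediately.
; Tick sets projectile speeds for one owner type and decrements the lifetime until destruction.
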(event Custom|KillMeOverTime
  ;[1 1 1] Kill Me Over time is for the lifetime of the bullets
  (Variables|Default|SetLifetime (- (Variables|Default|GetLifetime) (Variables|Default|GetLocalTick)))
  (if (<= (Variables|Default|GetLifetime) 0.0)
    (Development|PrintString "Bullet Died")
    (Actor|DestroyActor)))

(event Collision|EventActorBeginOverlap
  (params (OtherActor :type Actor%20Object%20Reference))
  (bind _returnvalue (Transformation|GetActorLocation OtherActor))
  (bind _damage (Variables|Default|GetDamage))
  ;[1 1 1] Event Hit
  (Development|PrintString "Eveent Begin Overlap")
  (Utilities|FlowControl|Sequence
    (:then_0
      (Utilities|Casting|CastToBP_MotionControllerLeft OtherActor
        (:CastFailed
          (Utilities|Casting|CastToBP_MotionControllerRight OtherActor
            (:CastFailed
              (Utilities|Casting|CastToBaseGun OtherActor
                (:CastFailed
                  (Utilities|FlowControl|Sequence
                    (:then_0
                      (bind _asbase_solider_ai (Utilities|Casting|CastToBaseSoliderAI OtherActor)
                        (:then
                          (if (not (Utilities|Enum|Equal(Enum) (Variables|Default|GetWhoOwnsMeBullet) "NewEnumerator1"))
                            (Development|PrintString "Hit Enemy")
                            (Default|TakeDamage _asbase_solider_ai _damage)
                            (Audio|PlaySoundatLocation OtherActor "/Game/Audio/Pre_10_26/VR_LazerGunImpact.VR_LazerGunImpact" _returnvalue "0, 0, 0" 1.0 1.0 0.0 0 0 0 :!label _label)
                            (Utilities|FlowControl|Sequence
                              (:then_0
                                (Effects|SpawnEmitteratLocation "/Game/StarterContent/Particles/P_Explosion.P_Explosion" _returnvalue))
                              (:then_1
                                (Class|GameplayStatics|SpawnDecalAttached "/Game/Materials/Red.Red" "2.000000,2.000000,2.000000" 0 "None" _returnvalue "0, 0, 0" "KeepRelativeOffset" 2.0)))))
                        (:CastFailed
                          (Development|PrintString "Hit Not Enemy")
                          (bind _asmotion_controller_pawn (Utilities|Casting|CastToMotionControllerPawn OtherActor)
                            (:then
                              (Development|PrintString "Hit Player")
                              (Default|TakeDamage _asmotion_controller_pawn _damage)
                              (Actor|DestroyActor)
                              (goto _label))
                            (:CastFailed
                              (goto _label))))))))))))))))

(event EventBeginPlay
  ;[1 1 1] Begin Play
  (Development|PrintString "Bullet Spawn"))

(event EventTick
  (params (DeltaSeconds :type Float%20%28single-precision%29))
  (bind _projectilemovement (Variables|Default|GetProjectileMovement))
  ;[1 1 1] Tick: Kill Me Overtime
  (Utilities|FlowControl|Sequence
    (:then_0
      (if (Utilities|Enum|Equal(Enum) (Variables|Default|GetWhoOwnsMeBullet) "NewEnumerator0")
        (Variables|/Script/Engine.ProjectileMovementComponent|SetInitialSpeed _projectilemovement 3e+03)
        (Variables|/Script/Engine.ProjectileMovementComponent|SetMaxSpeed _projectilemovement 6e+03)))
    (:then_1
      (Variables|Default|SetLocalTick DeltaSeconds)
      (CallFunction|KillMeOverTime))))

(event Collision|EventHit
  (params (MyComp :type Primitive%20Component%20Object%20Reference) (Other :type Actor%20Object%20Reference) (OtherComp :type Primitive%20Component%20Object%20Reference) (bSelfMoved :type Boolean) (HitLocation :type Vector :default "0, 0, 0") (HitNormal :type Vector :default "0, 0, 0") (NormalImpulse :type Vector :default "0, 0, 0") (Hit :type Hit%20Result%20Structure%20%28by%20ref%29))
  (bind _damage (Variables|Default|GetDamage))
  ;[1 1 1] Event Hit
  (Development|PrintString "Event Hit")
  (Utilities|FlowControl|Sequence
    (:then_0
      (Utilities|Casting|CastToBP_MotionControllerLeft (stale Collision|EventActorBeginOverlap OtherActor)
        (:CastFailed
          (Utilities|Casting|CastToBP_MotionControllerRight (stale Collision|EventActorBeginOverlap OtherActor)
            (:CastFailed
              (Utilities|Casting|CastToBaseGun (stale Collision|EventActorBeginOverlap OtherActor)
                (:CastFailed
                  (Utilities|FlowControl|Sequence
                    (:then_0
                      (bind _asbase_solider_ai (Utilities|Casting|CastToBaseSoliderAI (stale Collision|EventActorBeginOverlap OtherActor))
                        (:then
                          (if (not (Utilities|Enum|Equal(Enum) (Variables|Default|GetWhoOwnsMeBullet) "NewEnumerator1"))
                            (Development|PrintString "Hit Enemy")
                            (Default|TakeDamage _asbase_solider_ai _damage)
                            (Audio|PlaySoundatLocation (stale Collision|EventActorBeginOverlap OtherActor) "/Game/Audio/Pre_10_26/VR_LazerGunImpact.VR_LazerGunImpact" (Transformation|GetActorLocation (stale Collision|EventActorBeginOverlap OtherActor)) "0, 0, 0" 1.0 1.0 0.0 0 0 0 :!label _label)
                            (Utilities|FlowControl|Sequence
                              (:then_0
                                (Effects|SpawnEmitteratLocation "/Game/StarterContent/Particles/P_Explosion.P_Explosion" (Transformation|GetActorLocation (stale Collision|EventActorBeginOverlap OtherActor))))
                              (:then_1
                                (Class|GameplayStatics|SpawnDecalAttached "/Game/Materials/Red.Red" "2.000000,2.000000,2.000000" 0 "None" (Transformation|GetActorLocation (stale Collision|EventActorBeginOverlap OtherActor)) "0, 0, 0" "KeepRelativeOffset" 2.0)))))
                        (:CastFailed
                          (Development|PrintString "Hit Not Enemy")
                          (bind _asmotion_controller_pawn (Utilities|Casting|CastToMotionControllerPawn (stale Collision|EventActorBeginOverlap OtherActor))
                            (:then
                              (Development|PrintString "Hit Player")
                              (Default|TakeDamage _asmotion_controller_pawn _damage)
                              (Actor|DestroyActor)
                              (goto _label))
                            (:CastFailed
                              (goto _label))))))))))))))))

(fn ConstructionScript)