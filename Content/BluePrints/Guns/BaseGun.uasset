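; BaseGun is a gun actor for player or enemy that spawns BaseBullet projectiles and can be shown or hidden.
; Player shots use ammo, trigger force feedback, audio and timeline kickback, then start a cooldown that Tick clears after a delay while a material parameter animates the recharge.
; Tick also line-traces to place a short-lived, distance-scaled red-dot decal and polls overlaps for menu buttons and a Shield-based anti-cheat that reddens the gun.
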(event Custom|ShootGun
  (bind _defaultsceneroot (Variables|Default|GetDefaultSceneRoot))
  (bind _relativelocation (Variables|/Script/Engine.SceneComponent|GetRelativeLocation _defaultsceneroot))
  (bind (_x _y _z) (Math|Vector|BreakVector _relativelocation))
  ;[1 1 1] Shoot Gun
  (Variables|Default|SetShowTutorialText false)
  (switch Utilities|FlowControl|Switch|SwitchonOwner (Variables|Default|GetWhoOwnsMeGun)
    (:NewEnumerator0
      (if (Variables|Default|GetcanShoot)
        (if true
          (Math|Integer|DecrementInt (Variables|Default|GetcurrentAmmo)
            (:%20%20
              (Game|Feedback|ClientPlayForceFeedback (Game|GetPlayerController 0) "/Game/BluePrints/Guns/ShootForceFeedback.ShootForceFeedback" false false "None")
              (Game|SpawnActorfromClass "/Game/BluePrints/Guns/BaseBullet.BaseBullet_C" (Transformation|GetWorldTransform (Variables|Default|GetBulletSpawnPoint)) "AlwaysSpawn" 0 1 0)
              (Variables|Default|SetcanShoot false)
              (CallFunction|GunCooldownRecharge)
              (bind _outactors (Actor|GetAllActorsOfClass "/Game/BluePrints/Game_Necessary/AudioManager.AudioManager_C"))
              (Default|VFXChanger (Utilities|Array|Get(acopy) _outactors) "GunChargeUp" (Math|Conversions|ToTransform(Vector) (Transformation|GetWorldLocation (Variables|Default|GetGunMesh))))
              (bind _kickbackcurve (Timeline|Kickback PlayFromStart)
                (:Update
                  (Transformation|SetActorRelativeLocation (Math|Vector|MakeVector _kickbackcurve _y _z))
                  (Utilities|FlowControl|DoOnce false))))))
        (else
          (Game|Feedback|ClientPlayForceFeedback (Game|GetPlayerController 0) "/Game/ControllerFailedShot.ControllerFailedShot" false false "None"))))
    (:NewEnumerator1
      ;[1 1 1] Enemy Shooting Gun
      (bind _returnvalue (Game|SpawnActorfromClass "/Game/BluePrints/Guns/BaseBullet.BaseBullet_C" (Transformation|GetWorldTransform (Variables|Default|GetBulletSpawnPoint)) "AlwaysSpawn" 0 1 0))
      (Variables|/Game/BluePrints/Guns/BaseBullet.BaseBullet_C|SetWhoOwnsMeBullet _returnvalue "NewEnumerator1"))))

(event Custom|RedDot
  ;[1 1 1] Red Dot Stuff
  (if (not (Variables|Default|GetICantShootForCutscene))
    (Rendering|SetVisibility (Variables|Default|GetRedDotSpot) true false)))

(event Custom|TurnOffRedDot
  ;[1 1 1] Red Dot Stuff
  (Rendering|SetVisibility (Variables|Default|GetRedDotSpot) false false))

(event Custom|ShowCooldown
  ;[1 1 1] Show Cooldown: The Spots color changes based on being able to shoot or not
)

(event Custom|Cheating
  ;[1 1 1] Cheating System and menu button animation activation
  (if (Variables|Default|GetUseCheatingSystem)
    (Rendering|Material|SetMaterial (Variables|Default|GetGunMesh) 0 "/Game/Materials/Red.Red")
    (Variables|Default|SetCheatingCanShoot false)))

(event Custom|End%20Cheating
  ;[1 1 1] Cheating System and menu button animation activation
  (Rendering|Material|SetMaterial (Variables|Default|GetGunMesh) 0 (Variables|Default|GetDefaultMaterial))
  (Variables|Default|SetCheatingCanShoot true))

(event Custom|DeactivateMe
  ;[1 1 1] Deactivate/ Activate Gun
  (switch Utilities|FlowControl|Switch|SwitchonOwner (Variables|Default|GetWhoOwnsMeGun)
    (:NewEnumerator0
      (Development|PrintString "Deactivate")
      (Variables|Default|SetHasSpawned false)
      (Rendering|SetVisibility (Variables|Default|GetDefaultSceneRoot) false true)
      (Collision|SetCollisionEnabled (Variables|Default|GetGunMesh) "NoCollision")
      (Variables|Default|SetICantShootForCutscene false))))

(event Custom|ActivateMe
  ;[1 1 1] Deactivate/ Activate Gun
  (if (not (Variables|Default|GetICantShootForCutscene))
    (if (not (Variables|Default|GetHasSpawned))
      (bind _outactors (Actor|GetAllActorsOfClass "/Game/BluePrints/Game_Necessary/AudioManager.AudioManager_C"))
      (Default|VFXChanger (Utilities|Array|Get(acopy) _outactors) "GunPickUp")
      (Variables|Default|SetHasSpawned true)
      (Rendering|SetVisibility (Variables|Default|GetDefaultSceneRoot) true true)
      (Collision|SetCollisionEnabled (Variables|Default|GetGunMesh) "QueryAndPhysics")
      (Variables|Default|SetICantShootForCutscene true))))

(event Custom|GunCooldownRecharge
  ;[1 1 1] RechargeMaterial
  (bind _rechargevalue (Timeline|Recharge PlayFromStart)
    (:Update
      (Rendering|Material|SetScalarParameterValueonMaterials (Variables|Default|GetGunCooldownSpot) "Height" (* _rechargevalue 3.0)))))

(event Custom|NotBrokenBeginOverlap
  ;[1 1 1] Cheating System and menu button animation activation
  (if (== (Utilities|GetClass (stale Collision|EventActorBeginOverlap OtherActor)) "/Game/BluePrints/UI_Stuff/MenuButton.MenuButton_C")
    (Utilities|Casting|CastToMenuButton (stale Collision|EventActorBeginOverlap OtherActor))
    (else
      (Utilities|Casting|CastToShield (stale Collision|EventActorBeginOverlap OtherActor))
      (CallFunction|Cheating))))

(event Custom|NotBrokenEndOverlap
  ;[1 1 1] Cheating System and menu button animation activation
  (if (== (Utilities|GetClass (stale Collision|EventActorEndOverlap OtherActor)) "/Game/BluePrints/UI_Stuff/MenuButton.MenuButton_C")
    (Utilities|Casting|CastToMenuButton (stale Collision|EventActorEndOverlap OtherActor))
    (else
      (Utilities|Casting|CastToShield (stale Collision|EventActorEndOverlap OtherActor))
      (CallFunction|EndCheating))))

(event EventTick
  (params (DeltaSeconds :type Float%20%28single-precision%29))
  (bind _bulletspawnpoint (Variables|Default|GetBulletSpawnPoint))
  (bind _returnvalue (Transformation|GetWorldLocation _bulletspawnpoint))
  ;[1 1 1] Raycast for red dot decal
  (Utilities|FlowControl|Sequence
    (:then_0
      (if (Variables|Default|GetICantShootForCutscene)
        (bind _outhit (Collision|LineTraceByChannel _returnvalue (+ _returnvalue (* (Transformation|GetActorForwardVector) 5e+03)) "TraceTypeQuery1" true 0 "None"))
        (Rendering|Decal|SpawnDecalatLocation "/Game/Materials/RedDotDecal.RedDotDecal" (Math|Vector|ClampVectorSize (Math|Conversions|ToVector(Float) (* (.Distance (Collision|BreakHitResult _outhit)) 0.04)) 3e+01 85.0) (.ImpactPoint (Collision|BreakHitResult _outhit)) (Math|Conversions|RotationFromXVector (.ImpactNormal (Collision|BreakHitResult _outhit))) (+ DeltaSeconds 0.01))))
    (:then_1
      ;[1 1 1] Tick
      (CallFunction|ShowCooldown)
      (Utilities|FlowControl|Sequence
        (:then_0
          (if (not (Variables|Default|GetcanShoot))
            (Utilities|FlowControl|Delay (Variables|Default|GetShootWaitTime))
            (Variables|Default|SetcanShoot true)))
        (:then_1
          (if (not (Variables|Default|GetShowTutorialText))
            (Rendering|SetVisibility (Variables|Default|GetTutorialText) false false)))))
    (:then_2
      (if (Collision|IsOverlappingActor (stale Collision|EventActorBeginOverlap OtherActor) :!class /Script/Engine.Actor)
        (if (== (Utilities|GetClass (stale Collision|EventActorBeginOverlap OtherActor)) "/Game/BluePrints/UI_Stuff/MenuButton.MenuButton_C")
          (Utilities|FlowControl|DoOnce false :!label _label
            (:Completed
              (Development|PrintString "begin")
              (CallFunction|NotBrokenBeginOverlap)
              (goto _label_2 Reset))))
        (elif (== (Utilities|GetClass (stale Collision|EventActorBeginOverlap OtherActor)) "/Game/BluePrints/UI_Stuff/MenuButton.MenuButton_C")
          (Utilities|FlowControl|DoOnce false :!label _label_2
            (:Completed
              (Development|PrintString "end")
              (CallFunction|NotBrokenEndOverlap)
              (goto _label Reset))))))))

(event EventBeginPlay
  ;[1 1 1] Set's The Red Dot with a Default Material
  (if (not (Variables|Default|GetforPickUp))
    (CallFunction|DeactivateMe)))

(event Collision|EventActorBeginOverlap
  (params (OtherActor :type Actor%20Object%20Reference))
  ;[1 1 1] Cheating System and menu button animation activation
)

(event Collision|EventActorEndOverlap
  (params (OtherActor :type Actor%20Object%20Reference))
  ;[1 1 1] Cheating System and menu button animation activation
)

(event Input|KeyboardEvents|3
  (params (Key :type Key%20Structure))
  ;[1 1 1] RechargeMaterial
  (:Pressed
    (bind _rechargevalue (Timeline|Recharge PlayFromStart)
      (:Update
        (Rendering|Material|SetScalarParameterValueonMaterials (Variables|Default|GetGunCooldownSpot) "Height" (* _rechargevalue 3.0))))))

(fn ConstructionScript)

(fn EnemyShootingGun
  (bind _returnvalue (Game|SpawnActorfromClass "/Game/BluePrints/Guns/BaseBullet.BaseBullet_C" (Transformation|GetWorldTransform (Variables|Default|GetBulletSpawnPoint)) "AlwaysSpawn" 0 1 0))
  (Variables|/Game/BluePrints/Guns/BaseBullet.BaseBullet_C|SetWhoOwnsMeBullet _returnvalue "NewEnumerator1"))