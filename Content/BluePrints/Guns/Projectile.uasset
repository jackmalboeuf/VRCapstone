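; Projectile Blueprint for guns that damages Shield actors it overlaps.
; On overlap, an exact class check and cast identify a Shield, whose Health is reduced directly by the projectile's Damage value.
; It prints the remaining health to screen and destroys itself; other overlapped actors are ignored.
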(event Collision|EventActorBeginOverlap
  (params (OtherActor :type Actor%20Object%20Reference))
  (if (== (Utilities|GetClass OtherActor) "/Game/BluePrints/Game_Necessary/Shield.Shield_C")
    (bind _asshield (Utilities|Casting|CastToShield OtherActor))
    (bind _output_get (Variables|/Game/BluePrints/Game_Necessary/Shield.Shield_C|SetHealth _asshield (- (Variables|/Game/BluePrints/Game_Necessary/Shield.Shield_C|GetHealth _asshield) (Variables|Default|GetDamage))))
    (Development|PrintString (Utilities|String|ToString(Float) _output_get))
    (Actor|DestroyActor)))

(fn ConstructionScript)