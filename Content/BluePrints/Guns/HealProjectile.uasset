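; HealProjectile is a gun projectile Blueprint that heals Towers and acts on Shields it overlaps.
; On overlap with an actor whose class is exactly Tower, it adds Healing to that Tower's Health.
; For an exact Shield, it instead subtracts Damage from the Shield's Cooldown.
; Both hits print the new value and destroy the projectile, while other actors are ignored.
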(event EventBeginPlay)

(event Collision|EventActorBeginOverlap
  (params (OtherActor :type Actor%20Object%20Reference))
  (bind _returnvalue (Utilities|GetClass OtherActor))
  (if (== _returnvalue "/Game/BluePrints/Tower.Tower_C")
    (bind _astower (Utilities|Casting|CastToTower OtherActor))
    (bind _output_get (Variables|/Game/BluePrints/Tower.Tower_C|SetHealth _astower (+ (Variables|/Game/BluePrints/Tower.Tower_C|GetHealth _astower) (Variables|Default|GetHealing))))
    (Development|PrintString (Utilities|String|ToString(Float) _output_get))
    (Actor|DestroyActor)
    (elif (== _returnvalue "/Game/BluePrints/Game_Necessary/Shield.Shield_C")
      (bind _asshield (Utilities|Casting|CastToShield OtherActor))
      (bind _output_get_2 (Variables|/Game/BluePrints/Game_Necessary/Shield.Shield_C|SetCooldown _asshield (- (Variables|/Game/BluePrints/Game_Necessary/Shield.Shield_C|GetCooldown _asshield) (Variables|Default|GetDamage))))
      (Development|PrintString (Utilities|String|ToString(Float) _output_get_2))
      (Actor|DestroyActor))))

(event EventTick
  (params (DeltaSeconds :type Float%20%28single-precision%29)))

(fn ConstructionScript
  (|CallParentFunction))