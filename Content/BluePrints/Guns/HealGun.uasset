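; HealGun is a gun Blueprint that fires HealBullet projectiles when its EnemyShootingGun event is called.
; The event spawns a bullet at the BulletSpawnPoint transform and sets its WhoOwnsMeBullet to a fixed enum value to mark ownership.
; It has no other active logic: BeginPlay, overlap and Tick are disabled, the construction script only calls its parent, and NewFunction_0 is empty.
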(event EventBeginPlay
  (|CallParentFunction) ; This node is disabled and will not be called.\nDrag off pins to build functionality.
)

(event Collision|EventActorBeginOverlap
  (params (OtherActor :type Actor%20Object%20Reference))
  (|CallParentFunction OtherActor) ; This node is disabled and will not be called.\nDrag off pins to build functionality.
)

(event EventTick
  (params (DeltaSeconds :type Float%20%28single-precision%29))
  (|CallParentFunction DeltaSeconds) ; This node is disabled and will not be called.\nDrag off pins to build functionality.
)

(event EventEnemyShootingGun
  (bind _returnvalue (Game|SpawnActorfromClass "/Game/BluePrints/Guns/HealBullet.HealBullet_C" (Transformation|GetWorldTransform (Variables|Default|GetBulletSpawnPoint)) "Undefined" 0 0))
  (Variables|/Game/BluePrints/Guns/BaseBullet.BaseBullet_C|SetWhoOwnsMeBullet _returnvalue "NewEnumerator1"))

(fn ConstructionScript
  (|CallParentFunction))

(fn NewFunction0)