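; GunCooldownSlider displays a gun's shot cooldown on a progress bar.
; Tick polls the gun's CanShoot flag, using a DoOnce to start a timeline once each time shooting becomes unavailable and re-arming it when shooting is available again.
; The timeline's play rate is the inverse of the gun's ShootWaitTime, and its Fill track drives the bar's percent.
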(event EventTick
  (params (DeltaSeconds :type Float%20%28single-precision%29))
  (bind _gun (Variables|Default|GetGun))
  (if (Variables|/Game/BluePrints/Guns/BaseGun.BaseGun_C|GetcanShoot _gun)
    (goto _label Reset)
    (else
      (Utilities|FlowControl|DoOnce false :!label _label
        (:Completed
          (Components|Timeline|SetPlayRate (Variables|Default|GetTimeline_0) (/ 1.0 (Variables|/Game/BluePrints/Guns/BaseGun.BaseGun_C|GetShootWaitTime _gun)))
          (bind _fill (Timeline|Timeline_0 PlayFromStart)
            (:Update
              (Progress|SetPercent (Variables|/Game/BluePrints/UI_Stuff/CooldownBar.CooldownBar_C|GetProgressBar_33 (Variables|Default|GetProgressBar)) _fill))))))))

(fn ConstructionScript)