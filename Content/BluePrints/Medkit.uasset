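; Medkit is a health pickup that the player collects by shooting it, restoring health on the MotionControllerPawn.
; On overlap, Heal accepts only a PlayerBullet, adds HealAmount capped at MaxHealth, destroys the bullet and spawns the EnemyDeathExplosion effect.
; DelayThenKill then clears HealthPackSpawned on the EnemyManager and destroys the medkit after a short delay.
; The pawn and manager are both found through GetAllActorsOfClass.
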(event Custom|DelayThenKill
  (bind _outactors (Actor|GetAllActorsOfClass "/Game/BluePrints/AI_Enemy_Stuff/EnemyManager.EnemyManager_C"))
  (Variables|/Game/BluePrints/AI_Enemy_Stuff/EnemyManager.EnemyManager_C|SethealthPackSpawned (Utilities|Array|Get(acopy) _outactors) false)
  (Utilities|FlowControl|Delay 0.2)
  (Actor|DestroyActor))

(event EventBeginPlay)

(event Collision|EventActorBeginOverlap
  (params (OtherActor :type Actor%20Object%20Reference))
  (Development|PrintString "NONBullet")
  (CallFunction|Heal OtherActor))

(event EventTick
  (params (DeltaSeconds :type Float%20%28single-precision%29)))

(fn ConstructionScript)

(fn Heal
  (params (Object :type Object%20Object%20Reference))
  (bind _asplayer_bullet (Utilities|Casting|CastToPlayerBullet Object))
  (Development|PrintString "Bullet")
  (bind _outactors (Actor|GetAllActorsOfClass "/Game/VirtualRealityBP/Blueprints/MotionControllerPawn.MotionControllerPawn_C"))
  (if (< (Variables|/Game/VirtualRealityBP/Blueprints/MotionControllerPawn.MotionControllerPawn_C|GetMaxHealth (Utilities|Array|Get(acopy) _outactors)) (+ (Variables|/Game/VirtualRealityBP/Blueprints/MotionControllerPawn.MotionControllerPawn_C|GetHealth (Utilities|Array|Get(acopy) _outactors)) (Variables|Default|GetHealAmount)))
    (Variables|/Game/VirtualRealityBP/Blueprints/MotionControllerPawn.MotionControllerPawn_C|SetHealth (Utilities|Array|Get(acopy) _outactors) (Variables|/Game/VirtualRealityBP/Blueprints/MotionControllerPawn.MotionControllerPawn_C|GetMaxHealth (Utilities|Array|Get(acopy) _outactors)))
    (else
      (Variables|/Game/VirtualRealityBP/Blueprints/MotionControllerPawn.MotionControllerPawn_C|SetHealth (Utilities|Array|Get(acopy) _outactors) (+ (Variables|/Game/VirtualRealityBP/Blueprints/MotionControllerPawn.MotionControllerPawn_C|GetHealth (Utilities|Array|Get(acopy) _outactors)) (Variables|Default|GetHealAmount)))))
  (Actor|DestroyActor _asplayer_bullet)
  (Niagara|SpawnSystematLocation "/Game/Particles/EnemyDeathExplosion.EnemyDeathExplosion" (Transformation|GetWorldLocation (Variables|Debug|GetStaticMeshComponent)))
  (CallFunction|DelayThenKill))