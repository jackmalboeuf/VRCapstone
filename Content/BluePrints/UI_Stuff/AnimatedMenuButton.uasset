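; An animated menu button actor that reacts to a gun moving into or out of it.
; When a BaseGun begins overlapping, its skeletal mesh plays the button animation once, and end overlap plays the reverse animation.
; The G and F keys also print "Hello" and play the forward animation, apparently as debug triggers.
; Disconnected branches hold an unused "RedDot" actor tag check for the same animations.
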(event Collision|EventActorBeginOverlap
  (params (OtherActor :type Actor%20Object%20Reference))
  (Utilities|Casting|CastToBaseGun OtherActor)
  (Components|Animation|PlayAnimation (Variables|SkeletalMeshActor|GetSkeletalMeshComponent) "/Game/Models/Import/MenuButtonAnimated_Anim.MenuButtonAnimated_Anim" false))

(event Collision|EventActorEndOverlap
  (params (OtherActor :type Actor%20Object%20Reference))
  (Utilities|Casting|CastToBaseGun OtherActor)
  (Components|Animation|PlayAnimation (Variables|SkeletalMeshActor|GetSkeletalMeshComponent) "/Game/Models/Import/MenuButtonReverse_Anim.MenuButtonReverse_Anim" false))

(event Input|KeyboardEvents|F
  (params (Key :type Key%20Structure))
  (:Pressed
    (Development|PrintString "Hello")
    (Components|Animation|PlayAnimation (Variables|SkeletalMeshActor|GetSkeletalMeshComponent) "/Game/Models/Import/MenuButtonAnimated_Anim.MenuButtonAnimated_Anim" false)))

(event Input|KeyboardEvents|G
  (params (Key :type Key%20Structure))
  (:Pressed
    (Development|PrintString "Hello")
    (Components|Animation|PlayAnimation (Variables|SkeletalMeshActor|GetSkeletalMeshComponent) "/Game/Models/Import/MenuButtonAnimated_Anim.MenuButtonAnimated_Anim" false)))

(fn ConstructionScript)