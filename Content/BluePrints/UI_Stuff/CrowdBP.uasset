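; CrowdBP is an actor that displays a randomized animated crowd through its CrowdWidget component's CrowdUI widget.
; On BeginPlay it gathers the widget's four images, then shuffles preset X-position and color arrays to place and tint each image on the canvas.
; The CrowdMovement animation loops endlessly from a random start time, so separate instances can differ in layout, color and motion phase.
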(event EventBeginPlay
  (bind _locationx (Variables|Default|GetLocationX))
  (bind _images (Variables|Default|GetImages))
  (bind _ascrowd_ui (Utilities|Casting|CastToCrowdUI (UserInterface|GetUserWidgetObject (Variables|Default|GetCrowdWidget))))
  (Utilities|Array|Add _images (Variables|/Game/BluePrints/UI_Stuff/CrowdUI.CrowdUI_C|GetImage_57 _ascrowd_ui))
  (Utilities|Array|Add _images (Variables|/Game/BluePrints/UI_Stuff/CrowdUI.CrowdUI_C|GetImage_58 _ascrowd_ui))
  (Utilities|Array|Add _images (Variables|/Game/BluePrints/UI_Stuff/CrowdUI.CrowdUI_C|GetImage_59 _ascrowd_ui))
  (Utilities|Array|Add _images (Variables|/Game/BluePrints/UI_Stuff/CrowdUI.CrowdUI_C|GetImage_60 _ascrowd_ui))
  (Utilities|Array|Shuffle _locationx)
  (Utilities|Array|Shuffle (Variables|Default|GetColors))
  (for (_array_element _array_index) _locationx
    (Class|CanvasPanelSlot|SetPosition (Class|WidgetLayoutLibrary|SlotasCanvasSlot (Utilities|Array|Get(acopy) (Variables|Default|GetImages) _array_index)) (Math|Vector2D|MakeVector2D _array_element 0.0))
    (Class|Image|SetBrushTintColor (Utilities|Array|Get(acopy) (Variables|Default|GetImages) _array_index) (Utilities|Array|Get(acopy) (Variables|Default|GetColors) _array_index)))
  (UserInterface|Animation|PlayAnimation _ascrowd_ui (Variables|/Game/BluePrints/UI_Stuff/CrowdUI.CrowdUI_C|GetCrowdMovement _ascrowd_ui) (Math|Random|RandomFloatinRange 0.0 1.0) 0 "Forward" 1.0))

(fn ConstructionScript)