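; 3D HUD Blueprint that drives a health bar UserWidget held in a widget component, showing damage and healing.
; TakeDamage lowers stored health, plays a shake animation and uses a timeline to slide both progress bars to the new percent, printing debug values.
; HealUI raises health and picks threshold colours, but its nested contradictory checks keep the restyle and reversed timeline from running.
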(event Custom|TakeDamage
  (params (DamageAmount :type Integer))
  (Development|PrintString "DamageUI")
  (Variables|Default|SetDamageTaken DamageAmount)
  (CallFunction|TakeUIDamage))

(event Custom|TakeUIDamage
  (Variables|Default|SetCurrentHealth (- (Variables|Default|GetCurrentHealth) (Variables|Default|GetDamageTaken)))
  (UserInterface|Animation|PlayAnimation (Variables|Default|GetHealthBarWidget) (Variables|/Game/BluePrints/UI_Stuff/HudHealthBar.HudHealthBar_C|GetDamageShake (stale EventBeginPlay _ashud_health_bar)) 0.0 1 "Forward" 1.0)
  ;[1 1 1] Slide down animation
  (bind _newtrack_0 (Timeline|Timeline_0 PlayFromStart)
    (:Update
      (Progress|SetPercent (Variables|/Game/BluePrints/UI_Stuff/HudHealthBar.HudHealthBar_C|GetProgressBar_25 (stale EventBeginPlay _ashud_health_bar)) (/ (+ (* _newtrack_0 (Math|Conversions|ToFloat(Integer) (Variables|Default|GetDamageTaken))) (Math|Conversions|ToFloat(Integer) (Variables|Default|GetCurrentHealth))) (Math|Conversions|ToFloat(Integer) (Variables|Default|GetMaxHealth))))
      (Development|PrintString (Utilities|String|ToString(Float) (/ (+ (* _newtrack_0 (Math|Conversions|ToFloat(Integer) (Variables|Default|GetDamageTaken))) (Math|Conversions|ToFloat(Integer) (Variables|Default|GetCurrentHealth))) (Math|Conversions|ToFloat(Integer) (Variables|Default|GetMaxHealth)))))
      (Development|PrintString (Utilities|String|ToString(Integer) (Variables|Default|GetCurrentHealth)))
      (Development|PrintString (Utilities|String|ToString(Float) (Variables|/Script/UMG.ProgressBar|GetPercent (Variables|/Game/BluePrints/UI_Stuff/HudHealthBar.HudHealthBar_C|GetProgressBar_25 (stale EventBeginPlay _ashud_health_bar))))))))

(event Custom|SetHealthBarColor
  (bind _backgroundcolor (Variables|Default|GetBackgroundColor))
  (bind _healthbarcolor (Variables|Default|GetHealthBarColor))
  (bind _slatecolor (Utilities|Struct|MakeSlateColor _healthbarcolor))
  (bind _slatecolor_2 (Utilities|Struct|MakeSlateColor _backgroundcolor))
  (bind _slatebrush (Utilities|Struct|MakeSlateBrush "(X=32.000000,Y=32.000000)" "(Left=0.000000,Top=0.000000,Right=0.000000,Bottom=0.000000)" _slatecolor_2 0 "Image" "NoTile" "NoMirror"))
  (Variables|/Script/UMG.ProgressBar|SetWidgetStyle (Variables|/Game/BluePrints/UI_Stuff/HudHealthBar.HudHealthBar_C|GetProgressBar_25 (stale EventBeginPlay _output_get)) (Utilities|Struct|MakeProgressBarStyle _slatebrush (Utilities|Struct|MakeSlateBrush "(X=32.000000,Y=32.000000)" "(Left=0.000000,Top=0.000000,Right=0.000000,Bottom=0.000000)" _slatecolor (Variables|/Game/BluePrints/UI_Stuff/HudHealthBar.HudHealthBar_C|GetProgressBar_25 (stale EventBeginPlay _output_get)) "Image" "NoTile" "NoMirror") "(ImageSize=(X=32.000000,Y=32.000000),Margin=(Left=0.000000,Top=0.000000,Right=0.000000,Bottom=0.000000),Tint=(R=1.000000,G=1.000000,B=1.000000,A=1.000000),TintColor=(SpecifiedColor=(R=1.000000,G=1.000000,B=1.000000,A=1.000000),ColorUseRule=UseColor_Specified),ResourceObject=None,ResourceName=\"\",UVRegion=(Min=(X=0.000000,Y=0.000000),Max=(X=0.000000,Y=0.000000),bIsValid=0),DrawAs=Image,Tiling=NoTile,Mirroring=NoMirror,ImageType=NoImage,bIsDynamicallyLoaded=False,bHasUObject=False)"))
  (Variables|/Script/UMG.ProgressBar|SetWidgetStyle (Variables|/Game/BluePrints/UI_Stuff/HudHealthBar.HudHealthBar_C|GetProgressBar_26 (stale EventBeginPlay _output_get)) (Utilities|Struct|MakeProgressBarStyle _slatebrush (Utilities|Struct|MakeSlateBrush "(X=32.000000,Y=32.000000)" "(Left=0.000000,Top=0.000000,Right=0.000000,Bottom=0.000000)" _slatecolor (Variables|/Game/BluePrints/UI_Stuff/HudHealthBar.HudHealthBar_C|GetProgressBar_26 (stale EventBeginPlay _output_get)) "Image" "NoTile" "NoMirror") "(ImageSize=(X=32.000000,Y=32.000000),Margin=(Left=0.000000,Top=0.000000,Right=0.000000,Bottom=0.000000),Tint=(R=1.000000,G=1.000000,B=1.000000,A=1.000000),TintColor=(SpecifiedColor=(R=1.000000,G=1.000000,B=1.000000,A=1.000000),ColorUseRule=UseColor_Specified),ResourceObject=None,ResourceName=\"\",UVRegion=(Min=(X=0.000000,Y=0.000000),Max=(X=0.000000,Y=0.000000),bIsValid=0),DrawAs=Image,Tiling=NoTile,Mirroring=NoMirror,ImageType=NoImage,bIsDynamicallyLoaded=False,bHasUObject=False)")))

(event Custom|HealUI
  (params (HealAmount :type Integer))
  (Variables|Default|SetDamageTaken HealAmount)
  (bind _output_get (Variables|Default|SetCurrentHealth (+ (Variables|Default|GetCurrentHealth) (Variables|Default|GetDamageTaken))))
  (if (> _output_get 20)
    (Variables|Default|SetHealthBarColor "(R=0.000000,G=0.901961,B=0.043137,A=1.000000)")
    (if (<= _output_get 20)
      (Variables|Default|SetHealthBarColor "(R=0.901961,G=0.145098,B=0.000000,A=1.000000)")
      (if (<= _output_get 10)
        (Variables|Default|SetHealthBarColor "(R=0.901961,G=0.000000,B=0.000000,A=1.000000)")
        (CallFunction|SetHealthBarColor)
        ;[1 1 1] Slide down animation
        (bind _newtrack_0 (Timeline|Timeline_0 ReverseFromEnd)
          (:Update
            (Progress|SetPercent (Variables|/Game/BluePrints/UI_Stuff/HudHealthBar.HudHealthBar_C|GetProgressBar_25 (stale EventBeginPlay _ashud_health_bar)) (/ (+ (* _newtrack_0 (Math|Conversions|ToFloat(Integer) (Variables|Default|GetDamageTaken))) (Math|Conversions|ToFloat(Integer) (Variables|Default|GetCurrentHealth))) (Math|Conversions|ToFloat(Integer) (Variables|Default|GetMaxHealth))))
            (Development|PrintString (Utilities|String|ToString(Float) (/ (+ (* _newtrack_0 (Math|Conversions|ToFloat(Integer) (Variables|Default|GetDamageTaken))) (Math|Conversions|ToFloat(Integer) (Variables|Default|GetCurrentHealth))) (Math|Conversions|ToFloat(Integer) (Variables|Default|GetMaxHealth)))))
            (Development|PrintString (Utilities|String|ToString(Integer) (Variables|Default|GetCurrentHealth)))
            (Development|PrintString (Utilities|String|ToString(Float) (Variables|/Script/UMG.ProgressBar|GetPercent (Variables|/Game/BluePrints/UI_Stuff/HudHealthBar.HudHealthBar_C|GetProgressBar_25 (stale EventBeginPlay _ashud_health_bar)))))))))))

(event EventBeginPlay
  (bind _ashud_health_bar (Utilities|Casting|CastToHudHealthBar (UserInterface|GetUserWidgetObject (Variables|Default|GetWidget))))
  (bind _output_get (Variables|Default|SetHealthBarWidget _ashud_health_bar)))

(fn ConstructionScript)