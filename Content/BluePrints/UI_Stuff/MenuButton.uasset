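; MenuButton is a VR menu button actor with configurable text that triggers a menu action when hit or overlapped by a BaseBullet, then destroys itself.
; Pointer raycast events, or debug-style F and G keys, play timelines that scale and slide the highlight, with a sound after highlighting.
; A ButtonType switch quits the game or calls GameManager tutorial, match, game and battle functions, sometimes destroying the parent actor.
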(event Custom|MenuButtonPressed
  ;[1 1 1] Menu Button Pressed
  (Development|PrintString "Menu Button was Pressed")
  (switch Utilities|FlowControl|Switch|SwitchonMenuOptions (Variables|Default|GetButtonType)
    (:NewEnumerator0
      ;[1 1 1] Menu: Start Tutorial
      (bind _outactors (Actor|GetAllActorsOfClass "/Game/BluePrints/Game_Necessary/GameManager.GameManager_C"))
      (Default|TitleDestroy (Utilities|Array|Get(acopy) _outactors)))
    (:NewEnumerator1
      ;[1 1 1] Menu: Quit Game
      (Game|QuitGame 0 "Quit"))
    (:NewEnumerator2
      ;[1 1 1] Menu: Start Match
      (bind _outactors_2 (Actor|GetAllActorsOfClass "/Game/BluePrints/Game_Necessary/GameManager.GameManager_C"))
      (Default|RestartFunction (Utilities|Array|Get(acopy) _outactors_2)))
    (:NewEnumerator3
      ;[1 1 1] Start Game
      (bind _outactors_3 (Actor|GetAllActorsOfClass "/Game/BluePrints/Game_Necessary/GameManager.GameManager_C"))
      (Default|StartGame (Utilities|Array|Get(acopy) _outactors_3))
      (Actor|DestroyActor (Actor|GetAttachParentActor)))
    (:NewEnumerator4
      ;[1 1 1] Next
      (Actor|DestroyActor (Actor|GetAttachParentActor))
      (bind _outactors_4 (Actor|GetAllActorsOfClass "/Game/BluePrints/Game_Necessary/GameManager.GameManager_C"))
      (Default|StartBattle (Utilities|Array|Get(acopy) _outactors_4)))))

(event Custom|PointerRaycastHit
  (bind _buttonhighlight (Variables|Default|GetButtonHighlight))
  (bind _menubuttonbasemesh (Variables|Default|GetMenuButtonBaseMesh))
  ;[1 1 1] Highlight
  (Variables|Default|SetUsingAnimation true)
  (bind (_direction _location _scale) (Timeline|Highlight PlayFromStart)
    (:Update
      (Transformation|SetWorldTransform _menubuttonbasemesh (Math|Transform|MakeTransform (Transformation|GetWorldLocation _menubuttonbasemesh) (Transformation|GetWorldRotation _menubuttonbasemesh) (Math|Conversions|ToVector(Float) _scale)) false false)
      (Transformation|SetRelativeTransform _buttonhighlight (Math|Transform|MakeTransform (Math|Vector|MakeVector _location 0.0 0.0) (Transformation|GetWorldRotation _buttonhighlight) (Math|Conversions|ToVector(Float) _scale)) false false))
    (:Finished
      (Variables|Default|SetUsingAnimation false)
      (Audio|PlaySoundatLocation "/Game/Audio/10_26/VR_Menu_Selection.VR_Menu_Selection" (Transformation|GetWorldLocation (Variables|Default|GetDefaultSceneRoot)) "0, 0, 0" 1.0 1.0 0.0 0 0 0))))

(event Custom|PointerRaycastNotHit
  (bind _menubuttonbasemesh (Variables|Default|GetMenuButtonBaseMesh))
  (bind _buttonhighlight (Variables|Default|GetButtonHighlight))
  ;[1 1 1] Unhighlight
  (bind (_direction _scale _location) (Timeline|UnHighlight PlayFromStart)
    (:Update
      (Transformation|SetWorldTransform _menubuttonbasemesh (Math|Transform|MakeTransform (Transformation|GetWorldLocation _menubuttonbasemesh) (Transformation|GetWorldRotation _menubuttonbasemesh) (Math|Conversions|ToVector(Float) _scale)) false false)
      (Transformation|SetRelativeTransform _buttonhighlight (Math|Transform|MakeTransform (Math|Vector|MakeVector _location 0.0 0.0) (Transformation|GetWorldRotation _buttonhighlight) (Math|Conversions|ToVector(Float) _scale)) false false))))

(event Collision|EventHit
  (params (MyComp :type Primitive%20Component%20Object%20Reference) (Other :type Actor%20Object%20Reference) (OtherComp :type Primitive%20Component%20Object%20Reference) (bSelfMoved :type Boolean) (HitLocation :type Vector :default "0, 0, 0") (HitNormal :type Vector :default "0, 0, 0") (NormalImpulse :type Vector :default "0, 0, 0") (Hit :type Hit%20Result%20Structure%20%28by%20ref%29))
  ;[1 1 1] HIT: Bullet Thing
  (CallFunction|MenuButtonPressed)
  (Actor|DestroyActor))

(event EventBeginPlay
  ;[1 1 1] Begin Play
  (bind _outactors (Actor|GetAllActorsOfClass "/Game/BluePrints/Game_Necessary/BlackBox.BlackBox_C"))
  (Variables|Default|SetBlackBox (Utilities|Array|Get(acopy) _outactors))
  (Rendering|Components|TextRender|SetText (Variables|Default|GetTextRender) (Utilities|Text|ToText(String) (Variables|Default|GetButtonText))))

(event Collision|EventActorBeginOverlap
  (params (OtherActor :type Actor%20Object%20Reference))
  ;[1 1 1] HIT: Bullet Thing
  (Utilities|Casting|CastToBaseBullet OtherActor)
  (CallFunction|MenuButtonPressed)
  (Actor|DestroyActor))

(event Input|KeyboardEvents|F
  (params (Key :type Key%20Structure))
  (bind _buttonhighlight (Variables|Default|GetButtonHighlight))
  (bind _menubuttonbasemesh (Variables|Default|GetMenuButtonBaseMesh))
  ;[1 1 1] Highlight
  (:Pressed
    (bind (_direction _location _scale) (Timeline|Highlight PlayFromStart)
      (:Update
        (Transformation|SetWorldTransform _menubuttonbasemesh (Math|Transform|MakeTransform (Transformation|GetWorldLocation _menubuttonbasemesh) (Transformation|GetWorldRotation _menubuttonbasemesh) (Math|Conversions|ToVector(Float) _scale)) false false)
        (Transformation|SetRelativeTransform _buttonhighlight (Math|Transform|MakeTransform (Math|Vector|MakeVector _location 0.0 0.0) (Transformation|GetWorldRotation _buttonhighlight) (Math|Conversions|ToVector(Float) _scale)) false false))
      (:Finished
        (Variables|Default|SetUsingAnimation false)
        (Audio|PlaySoundatLocation "/Game/Audio/10_26/VR_Menu_Selection.VR_Menu_Selection" (Transformation|GetWorldLocation (Variables|Default|GetDefaultSceneRoot)) "0, 0, 0" 1.0 1.0 0.0 0 0 0)))))

(event Input|KeyboardEvents|Y
  (params (Key :type Key%20Structure)))

(event Input|KeyboardEvents|G
  (params (Key :type Key%20Structure))
  (bind _menubuttonbasemesh (Variables|Default|GetMenuButtonBaseMesh))
  (bind _buttonhighlight (Variables|Default|GetButtonHighlight))
  ;[1 1 1] Unhighlight
  (:Pressed
    (bind (_direction _scale _location) (Timeline|UnHighlight PlayFromStart)
      (:Update
        (Transformation|SetWorldTransform _menubuttonbasemesh (Math|Transform|MakeTransform (Transformation|GetWorldLocation _menubuttonbasemesh) (Transformation|GetWorldRotation _menubuttonbasemesh) (Math|Conversions|ToVector(Float) _scale)) false false)
        (Transformation|SetRelativeTransform _buttonhighlight (Math|Transform|MakeTransform (Math|Vector|MakeVector _location 0.0 0.0) (Transformation|GetWorldRotation _buttonhighlight) (Math|Conversions|ToVector(Float) _scale)) false false)))))

(fn ConstructionScript)