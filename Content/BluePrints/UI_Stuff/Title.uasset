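; Title actor for a VR game that briefly shows a static mesh and two text renders, then removes itself.
; All three components start hidden on BeginPlay.
; The SpawnTitle event reveals them immediately, while an overlap by the MotionControllerPawn leads into the same reveal after a fixed delay.
; Once revealed, the title stays up for a few seconds before the actor destroys itself.
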(event Custom|SpawnTitle
  (bind _staticmeshcomponent (Variables|Debug|GetStaticMeshComponent))
  (Development|SetHiddeninGame _staticmeshcomponent false false)
  (Rendering|SetVisibility _staticmeshcomponent true false)
  (Utilities|FlowControl|Delay 5.0)
  (Actor|DestroyActor))

(event EventBeginPlay
  (Development|SetHiddeninGame (Variables|Default|GetTextRender2) true false))

(event Collision|EventActorBeginOverlap
  (params (OtherActor :type Actor%20Object%20Reference))
  (bind _staticmeshcomponent (Variables|Debug|GetStaticMeshComponent))
  (Utilities|Casting|CastToMotionControllerPawn OtherActor)
  (Utilities|FlowControl|Delay 14.0)
  (Development|SetHiddeninGame _staticmeshcomponent false false)
  (Rendering|SetVisibility _staticmeshcomponent true false)
  (Utilities|FlowControl|Delay 5.0)
  (Actor|DestroyActor))

(fn ConstructionScript)