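; Test game manager for a two-player, turn-based board game that cycles each turn through Start, Draw, Play, Action and End phases.
; SpaceBar advances the phase, and ending a turn hands play to the other player.
; Phase changes mirror to the first MotionControllerPawn on Player 1's turn, and both turn starts reset it to Start.
; BeginPlay assigns BoardTiles owners, rows and columns through a hard-coded index switch.
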(event Custom|Start%20Player%201%20Turn
  ;[1 1 1] Start The Others Turn
  (Variables|Default|SetWhoseTurnIsIt "NewEnumerator0")
  (Development|PrintString "Player 1 Turn")
  (Variables|/Game/VirtualRealityBP/Blueprints/MotionControllerPawn.MotionControllerPawn_C|SetTurnPhase (Variables|Default|GetPlayer) "NewEnumerator0")
  (Variables|Default|SetCurrentTurnPhase "NewEnumerator0"))

(event Custom|Start%20Player%202%20Turn
  ;[1 1 1] Start The Others Turn
  (Variables|Default|SetWhoseTurnIsIt "NewEnumerator1")
  (Development|PrintString "Player 2 Turn")
  (Variables|/Game/VirtualRealityBP/Blueprints/MotionControllerPawn.MotionControllerPawn_C|SetTurnPhase (Variables|Default|GetPlayer) "NewEnumerator0")
  (Variables|Default|SetCurrentTurnPhase "NewEnumerator0"))

(event Custom|EndTurn
  ;[1 1 1] End Turn
  (switch Utilities|FlowControl|Switch|SwitchonCurrentTurn (Variables|Default|GetWhoseTurnIsIt)
    (:NewEnumerator0
      (CallFunction|StartPlayer2Turn))
    (:NewEnumerator1
      (CallFunction|StartPlayer1Turn))))

(event Custom|GoToNextPhase
  ;[1 1 1] Way to Jump Phases
  (switch Utilities|FlowControl|Switch|SwitchonTurnPhases (Variables|Default|GetCurrentTurnPhase)
    (:NewEnumerator0
      (CallFunction|DrawPhase))
    (:NewEnumerator1
      (CallFunction|PlayPhase))
    (:NewEnumerator2
      (CallFunction|ActionPhase))
    (:NewEnumerator3
      (CallFunction|EndPhase))
    (:NewEnumerator4
      (CallFunction|EndTurn))))

(event Custom|StartPhase
  ;[1 1 1] The Actual Phases
  (Development|PrintString "Start Phase")
  (Variables|Default|SetCurrentTurnPhase "NewEnumerator0")
  (switch Utilities|FlowControl|Switch|SwitchonCurrentTurn (Variables|Default|GetWhoseTurnIsIt)
    (:NewEnumerator0
      (Variables|/Game/VirtualRealityBP/Blueprints/MotionControllerPawn.MotionControllerPawn_C|SetTurnPhase (Variables|Default|GetPlayer) "NewEnumerator0"))))

(event Custom|DrawPhase
  ;[1 1 1] The Actual Phases
  (Development|PrintString "Draw Phase")
  (Variables|Default|SetCurrentTurnPhase "NewEnumerator1")
  (switch Utilities|FlowControl|Switch|SwitchonCurrentTurn (Variables|Default|GetWhoseTurnIsIt)
    (:NewEnumerator0
      (Variables|/Game/VirtualRealityBP/Blueprints/MotionControllerPawn.MotionControllerPawn_C|SetTurnPhase (Variables|Default|GetPlayer) "NewEnumerator1"))))

(event Custom|PlayPhase
  ;[1 1 1] The Actual Phases
  (Development|PrintString "Play Phase")
  (Variables|Default|SetCurrentTurnPhase "NewEnumerator2")
  (switch Utilities|FlowControl|Switch|SwitchonCurrentTurn (Variables|Default|GetWhoseTurnIsIt)
    (:NewEnumerator0
      (Variables|/Game/VirtualRealityBP/Blueprints/MotionControllerPawn.MotionControllerPawn_C|SetTurnPhase (Variables|Default|GetPlayer) "NewEnumerator2"))))

(event Custom|ActionPhase
  ;[1 1 1] The Actual Phases
  (Development|PrintString "Action Phase")
  (Variables|Default|SetCurrentTurnPhase "NewEnumerator3")
  (switch Utilities|FlowControl|Switch|SwitchonCurrentTurn (Variables|Default|GetWhoseTurnIsIt)
    (:NewEnumerator0
      (Variables|/Game/VirtualRealityBP/Blueprints/MotionControllerPawn.MotionControllerPawn_C|SetTurnPhase (Variables|Default|GetPlayer) "NewEnumerator3"))))

(event Custom|EndPhase
  ;[1 1 1] The Actual Phases
  (Development|PrintString "End Phase")
  (Variables|Default|SetCurrentTurnPhase "NewEnumerator4")
  (switch Utilities|FlowControl|Switch|SwitchonCurrentTurn (Variables|Default|GetWhoseTurnIsIt)
    (:NewEnumerator0
      (Variables|/Game/VirtualRealityBP/Blueprints/MotionControllerPawn.MotionControllerPawn_C|SetTurnPhase (Variables|Default|GetPlayer) "NewEnumerator4"))))

(event Custom|Set%20Owners
  ;[1 1 1] UGLY Way to Set Tiles for Right Now
  (for (_array_element _array_index) (Variables|Default|GetBoardTiles)
    (switch int _array_index
      (:0
        (Default|SetPlayer1asOwner _array_element)
        (Default|SetLocationasColumn1 _array_element)
        (Default|SetLocationasRow1 _array_element))
      (:1
        (Default|SetPlayer1asOwner _array_element)
        (Default|SetLocationasColumn2 _array_element)
        (Default|SetLocationasRow1 _array_element))
      (:2
        (Default|SetPlayer1asOwner _array_element)
        (Default|SetLocationasColumn3 _array_element)
        (Default|SetLocationasRow1 _array_element))
      (:3
        (Default|SetPlayer1asOwner _array_element)
        (Default|SetLocationasColumn1 _array_element)
        (Default|SetLocationasRow2 _array_element))
      (:4
        (Default|SetPlayer1asOwner _array_element)
        (Default|SetLocationasColumn2 _array_element)
        (Default|SetLocationasRow2 _array_element))
      (:5
        (Default|SetPlayer1asOwner _array_element)
        (Default|SetLocationasColumn3 _array_element)
        (Default|SetLocationasRow2 _array_element))
      (:6
        (Default|SetPlayer2asOwner _array_element)
        (Default|SetLocationasColumn1 _array_element)
        (Default|SetLocationasRow3 _array_element))
      (:7
        (Default|SetPlayer2asOwner _array_element)
        (Default|SetLocationasColumn2 _array_element)
        (Default|SetLocationasRow3 _array_element))
      (:8
        (Default|SetPlayer2asOwner _array_element)
        (Default|SetLocationasColumn3 _array_element)
        (Default|SetLocationasRow3 _array_element))
      (:9
        (Default|SetPlayer2asOwner _array_element)
        (Default|SetLocationasColumn1 _array_element)
        (Default|SetLocationasRow4 _array_element))
      (:10
        (Default|SetPlayer2asOwner _array_element)
        (Default|SetLocationasColumn2 _array_element)
        (Default|SetLocationasRow4 _array_element))
      (:11
        (Default|SetPlayer2asOwner _array_element)
        (Default|SetLocationasColumn3 _array_element)
        (Default|SetLocationasRow4 _array_element)))))

(event EventBeginPlay
  (bind _outactors (Actor|GetAllActorsOfClass "/Game/VirtualRealityBP/Blueprints/MotionControllerPawn.MotionControllerPawn_C"))
  (Variables|Default|SetPlayer (Utilities|Array|Get(acopy) _outactors))
  (CallFunction|SetOwners))

(event Input|KeyboardEvents|SpaceBar
  (params (Key :type Key%20Structure))
  (:Pressed
    (Development|PrintString "Go To Next Phase")
    (CallFunction|GotoNextPhase)))

(fn ConstructionScript)